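; BP_Manager_Cinematics is a manager Blueprint that switches between the cinematic and main cameras via numpad keys.
; Shortly after BeginPlay it enables input from the first player controller.
; Its events forward switch-to-cine, switch-to-main and toggle requests to CameraWorldSubsystem after a validity check.
; The toggle key also prints an on-screen message.
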(event `self.ReceiveBeginPlay`
  (bind _returnvalue (`GameplayStatics.GetPlayerController` 0))
  ;[0.4735 1 0.5174] Begin Play
  (`KismetSystemLibrary.Delay` 0.2)
  (`/Engine/EditorBlueprintResources/StandardMacros.IsValid` _returnvalue
    (:`Is Valid`
      (`self.EnableInput` _returnvalue))))

(event `ToCineCamera`
  (bind _returnvalue (subsystem `CameraWorldSubsystem`))
  ;[1 1 1] Siwth Camera
  (`/Engine/EditorBlueprintResources/StandardMacros.IsValid` _returnvalue
    (:`Is Valid`
      (`CameraWorldSubsystem.SwitchToCineCamera` _returnvalue))))

(event `ToMainCamera`
  (bind _returnvalue (subsystem `CameraWorldSubsystem`))
  ;[1 1 1] Siwth Camera
  (`/Engine/EditorBlueprintResources/StandardMacros.IsValid` _returnvalue
    (:`Is Valid`
      (`CameraWorldSubsystem.SwitchToMainCamera` _returnvalue))))

(event `CE_ToggleCamera`
  (bind _returnvalue (subsystem `CameraWorldSubsystem`))
  ;[1 1 1] Toggle Camera
  (`/Engine/EditorBlueprintResources/StandardMacros.IsValid` _returnvalue
    (:`Is Valid`
      (`CameraWorldSubsystem.ToggleCameraTarget` _returnvalue))))

(event `Key|NumPadZero`
  (params (Key :type "Key Structure"))
  ;[1 1 1] Input Events
  (:`Pressed`
    (`self.CE_ToggleCamera`)
    (`KismetSystemLibrary.PrintString` "Toggle" true true (struct :`R` 1.0 :`G` 0.627358 :`B` 0.321704 :`A` 1.0))))

(event `Key|NumPadOne`
  (params (Key :type "Key Structure"))
  ;[1 1 1] Input Events
  (:`Pressed`
    (`self.ToCineCamera`)))

(event `Key|NumPadTwo`
  (params (Key :type "Key Structure"))
  ;[1 1 1] Input Events
  (:`Pressed`
    (`self.ToMainCamera`)))

(fn `UserConstructionScript`)