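; BP_PillarZone is a pillar zone that gives visual feedback on its associated pillar by recoloring a spotlight.
; Events for pillar grab, ungrab, enable, disable and zone show set the light to grabbed, move or base color.
; Ungrab and disable pick the move color while the zone state is Moving, otherwise base; enable and show always use base.
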(event `self.OnReceiveAssociatedPillarGrabbed`
  (bind _spotlightcomponent (`self.SpotLightComponent`))
  ;[1 0.3813 0.9387] Associated Pillar Grabbed
  (`|ExecutionSequence`
    (:`then_0`
      (`/Engine/EditorBlueprintResources/StandardMacros.IsValid` _spotlightcomponent
        (:`Is Valid`
          (`LightComponent.SetLightColor` _spotlightcomponent (`self.ColorGrabbed`) true))))))

(event `self.OnReceiveAssociatedPillarUnGrabbed`
  (bind _spotlightcomponent (`self.SpotLightComponent`))
  ;[1 0.3813 0.9387] Associated Pillar Ungrabbed
  (`|ExecutionSequence`
    (:`then_0`
      (`/Engine/EditorBlueprintResources/StandardMacros.IsValid` _spotlightcomponent
        (:`Is Valid`
          (if (`|EnumEquality` (`self.CurrentZoneState`) "Moving")
            (`LightComponent.SetLightColor` _spotlightcomponent (`self.ColorMove`) true)
            (else
              (`LightComponent.SetLightColor` _spotlightcomponent (`self.ColorBase`) true))))))))

(event `self.ReceiveOnShowZone`
  (bind _spotlightcomponent (`self.SpotLightComponent`))
  ;[1 0.3813 0.9387] OnShow Zone
  (`KismetSystemLibrary.PrintString` "on show zone")
  (`|ExecutionSequence`
    (:`then_0`
      (`/Engine/EditorBlueprintResources/StandardMacros.IsValid` _spotlightcomponent
        (:`Is Valid`
          (`LightComponent.SetLightColor` _spotlightcomponent (`self.ColorBase`) true))))))

(event `self.OnReceiveDisablePillar`
  (bind _spotlightcomponent (`self.SpotLightComponent`))
  (`/Engine/EditorBlueprintResources/StandardMacros.IsValid` _spotlightcomponent
    (:`Is Valid`
      (if (`|EnumEquality` (`self.CurrentZoneState`) "Moving")
        (`LightComponent.SetLightColor` _spotlightcomponent (`self.ColorMove`) true)
        (else
          (`LightComponent.SetLightColor` _spotlightcomponent (`self.ColorBase`) true))))))

(event `self.OnReceiveEnablePillar`
  (bind _spotlightcomponent (`self.SpotLightComponent`))
  (`/Engine/EditorBlueprintResources/StandardMacros.IsValid` _spotlightcomponent
    (:`Is Valid`
      (`LightComponent.SetLightColor` _spotlightcomponent (`self.ColorBase`) true))))

(fn `UserConstructionScript`)