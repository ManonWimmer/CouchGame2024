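; BP_PowerUp_Duck is the collectible duck power-up, animated while idle and when picked.
; On BeginPlay it configures four juiciness animation components from DuckAnimData, then starts the rotate, scale-appear and bobbing effects.
; CollectDuck plays the pick sound through the sound subsystem, stops those three effects, runs the pick animation and activates the pickup VFX.
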(event `CE_InitAnims`
  (bind _duckanimdata (`self.DuckAnimData`))
  (bind _duckanimdata_2 (`self.DuckAnimData`))
  (bind _duckanimdata_3 (`self.DuckAnimData`))
  (bind _bpc_juicinessanim_rotateinfinite (`self.BPC_JuicinessAnim_RotateInfinite`))
  (bind _bpc_juicinessanim_pickeffect (`self.BPC_JuicinessAnim_PickEffect`))
  (bind _bpc_juicinessanim_scaleappear (`self.BPC_JuicinessAnim_ScaleAppear`))
  (bind _bpc_juicinessanim_bobbingeffect (`self.BPC_JuicinessAnim_BobbingEffect`))
  ;[0.3704 0.4644 1] Init Anims
  (`/Engine/EditorBlueprintResources/StandardMacros.IsValid` (`self.DuckAnimData`)
    (:`Is Valid`
      (`|ExecutionSequence`
        (:`then_0`
          (`/Engine/EditorBlueprintResources/StandardMacros.IsValid` _bpc_juicinessanim_rotateinfinite
            (:`Is Valid`
              (`/Game/Project/Blueprints/JuicinessAnimComponents/RotateInfinite/BPC_JuicinessAnim_RotateInfinite.CE_InitAnim` _bpc_juicinessanim_rotateinfinite (`JuicinessAnimData.RotateInfiniteDuckRandomDelayMax` _duckanimdata_2) (`JuicinessAnimData.RotateInfiniteDuckDuration` _duckanimdata_2)))))
        (:`then_1`
          (`/Engine/EditorBlueprintResources/StandardMacros.IsValid` _bpc_juicinessanim_pickeffect
            (:`Is Valid`
              (`/Game/Project/Blueprints/JuicinessAnimComponents/PickEffect/BPC_JuicinessAnim_PickEffect.CE_InitAnim` _bpc_juicinessanim_pickeffect (`JuicinessAnimData.PickDuckRotateDuration` _duckanimdata_3) (`JuicinessAnimData.PickJumpDuckDuration` _duckanimdata_3) (`JuicinessAnimData.PickDuckTargetScaleDivider` _duckanimdata_3)))))
        (:`then_2`
          (`/Engine/EditorBlueprintResources/StandardMacros.IsValid` _bpc_juicinessanim_scaleappear
            (:`Is Valid`
              (`/Game/Project/Blueprints/JuicinessAnimComponents/ScaleAppear/BPC_JuicinessAnim_ScaleAppear.CE_InitAnim` _bpc_juicinessanim_scaleappear (`JuicinessAnimData.ScaleAppearDuckDuration` (`self.DuckAnimData`))))))
        (:`then_3`
          (`/Engine/EditorBlueprintResources/StandardMacros.IsValid` _bpc_juicinessanim_bobbingeffect
            (:`Is Valid`
              (`/Game/Project/Blueprints/JuicinessAnimComponents/BobbingEffect/BPC_JuicinessAnim_BobbingEffect.CE_InitAnim` _bpc_juicinessanim_bobbingeffect (`JuicinessAnimData.DuckBobbingDuration` _duckanimdata) (`JuicinessAnimData.DuckBobbingOffset` _duckanimdata) (`JuicinessAnimData.DuckBobbingRandomDelayMax` _duckanimdata)))))))))

(event `self.ReceiveBeginPlay`
  (bind _bpc_juicinessanim_scaleappear (`self.BPC_JuicinessAnim_ScaleAppear`))
  (bind _bpc_juicinessanim_bobbingeffect (`self.BPC_JuicinessAnim_BobbingEffect`))
  (bind _bpc_juicinessanim_rotateinfinite (`self.BPC_JuicinessAnim_RotateInfinite`))
  ;[0.4065 1 0.2367] Begin Play
  (`|ExecutionSequence`
    (:`then_0`
      (`self.CE_InitAnims`))
    (:`then_1`
      (`/Engine/EditorBlueprintResources/StandardMacros.IsValid` _bpc_juicinessanim_rotateinfinite
        (:`Is Valid`
          (`/Game/Project/Blueprints/JuicinessAnimComponents/RotateInfinite/BPC_JuicinessAnim_RotateInfinite.CE_StartAnim` _bpc_juicinessanim_rotateinfinite))))
    (:`then_2`
      (`/Engine/EditorBlueprintResources/StandardMacros.IsValid` _bpc_juicinessanim_scaleappear
        (:`Is Valid`
          (`/Game/Project/Blueprints/JuicinessAnimComponents/ScaleAppear/BPC_JuicinessAnim_ScaleAppear.CE_StartAnim` _bpc_juicinessanim_scaleappear))))
    (:`then_3`
      (`/Engine/EditorBlueprintResources/StandardMacros.IsValid` _bpc_juicinessanim_bobbingeffect
        (:`Is Valid`
          (`/Game/Project/Blueprints/JuicinessAnimComponents/BobbingEffect/BPC_JuicinessAnim_BobbingEffect.CE_StartAnim` _bpc_juicinessanim_bobbingeffect))))))

(event `self.ReceiveCollectDuck`
  (bind _returnvalue (subsystem `SoundSubsystem`))
  (bind _bpc_juicinessanim_pickeffect (`self.BPC_JuicinessAnim_PickEffect`))
  (bind _bpc_juicinessanim_scaleappear (`self.BPC_JuicinessAnim_ScaleAppear`))
  (bind _bpc_juicinessanim_bobbingeffect (`self.BPC_JuicinessAnim_BobbingEffect`))
  (bind _bpc_juicinessanim_rotateinfinite (`self.BPC_JuicinessAnim_RotateInfinite`))
  ;[1 0.5051 0.8411] Collect Duck
  (`|ExecutionSequence`
    (:`then_0`
      (`/Engine/EditorBlueprintResources/StandardMacros.IsValid` _returnvalue
        (:`Is Valid`
          (`SoundSubsystem.PlayDuckPickSound` _returnvalue))))
    (:`then_1`
      (`/Engine/EditorBlueprintResources/StandardMacros.IsValid` _bpc_juicinessanim_bobbingeffect
        (:`Is Valid`
          (`/Game/Project/Blueprints/JuicinessAnimComponents/BobbingEffect/BPC_JuicinessAnim_BobbingEffect.CE_StopAnim` _bpc_juicinessanim_bobbingeffect))))
    (:`then_2`
      (`/Engine/EditorBlueprintResources/StandardMacros.IsValid` _bpc_juicinessanim_rotateinfinite
        (:`Is Valid`
          (`/Game/Project/Blueprints/JuicinessAnimComponents/RotateInfinite/BPC_JuicinessAnim_RotateInfinite.CE_StopAnim` _bpc_juicinessanim_rotateinfinite))))
    (:`then_3`
      (`/Engine/EditorBlueprintResources/StandardMacros.IsValid` _bpc_juicinessanim_scaleappear
        (:`Is Valid`
          (`/Game/Project/Blueprints/JuicinessAnimComponents/ScaleAppear/BPC_JuicinessAnim_ScaleAppear.CE_StopAnim` _bpc_juicinessanim_scaleappear))))
    (:`then_4`
      (`/Engine/EditorBlueprintResources/StandardMacros.IsValid` _bpc_juicinessanim_pickeffect
        (:`Is Valid`
          (`/Game/Project/Blueprints/JuicinessAnimComponents/PickEffect/BPC_JuicinessAnim_PickEffect.CE_PickAnim` _bpc_juicinessanim_pickeffect))))
    (:`then_5`
      (`/Engine/EditorBlueprintResources/StandardMacros.IsValid` null
        (:`Is Valid`
          (`ActorComponent.Activate` (`self.VFX_PickUp`) false))))))

(fn `UserConstructionScript`)