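; BP_Manager_Events is an event manager Blueprint that handles audio and fireworks feedback for the game's round events.
; When phase 2 of an event triggers, it plays the fireworks sound and fires all fireworks through the Sound and Fireworks subsystems.
; Round phase changes stop fireworks at pre-round, and at round start pick in-game music by the current event name (Duck, Zones, Mole or Push), printing a debug string.
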(event `self.ReceiveOnTriggerEventPhase2`
  (bind _returnvalue (subsystem `FireworksSubsystem`))
  (bind _returnvalue_2 (subsystem `SoundSubsystem`))
  ;[0.8919 0.3575 1] On Trigger Event Phase 2
  (`|ExecutionSequence`
    (:`then_0`
      (`/Engine/EditorBlueprintResources/StandardMacros.IsValid` _returnvalue_2
        (:`Is Valid`
          (`SoundSubsystem.PlayFireworksSound` _returnvalue_2))))
    (:`then_1`
      (`/Engine/EditorBlueprintResources/StandardMacros.IsValid` _returnvalue
        (:`Is Valid`
          (`FireworksSubsystem.FireAllFireworks` _returnvalue))))))

(event `self.ReceiveCheckNewPhase`
  (params (InRoundsPhaseID :type "ERoundsPhaseID Enum" :default "NONE"))
  (bind _returnvalue (`self.GetCurrentEventData`))
  (bind _returnvalue_2 (subsystem `FireworksSubsystem`))
  (bind _returnvalue_3 (subsystem `SoundSubsystem`))
  (bind _returnvalue_4 (subsystem `SoundSubsystem`))
  (bind _returnvalue_5 (subsystem `SoundSubsystem`))
  (bind _returnvalue_6 (subsystem `SoundSubsystem`))
  ;[0.8919 0.3575 1] Play music round at starting round
  (switch `ERoundsPhaseID` InRoundsPhaseID
    (:`PRE_ROUND`
      ;[0.8919 0.3575 1] Pre Round -> stop fireworks
      (`/Engine/EditorBlueprintResources/StandardMacros.IsValid` _returnvalue_2
        (:`Is Valid`
          (`FireworksSubsystem.StopAllFireworks` _returnvalue_2))))
    (:`STARTING_ROUND`
      (`/Engine/EditorBlueprintResources/StandardMacros.IsValid` _returnvalue
        (:`Is Valid`
          (switch `EEventName` (`EventData.EventName` _returnvalue)
            (:`Duck`
              (`/Engine/EditorBlueprintResources/StandardMacros.IsValid` _returnvalue_4
                (:`Is Valid`
                  (`SoundSubsystem.PlayInGameDuckMusicSound` _returnvalue_4)
                  (`KismetSystemLibrary.PrintString` "Play Duck Music"))))
            (:`Zones`
              (`/Engine/EditorBlueprintResources/StandardMacros.IsValid` _returnvalue_5
                (:`Is Valid`
                  (`SoundSubsystem.PlayInGamePopcornMusicSound` _returnvalue_5)
                  (`KismetSystemLibrary.PrintString` "Play Zones Music"))))
            (:`Mole`
              (`/Engine/EditorBlueprintResources/StandardMacros.IsValid` _returnvalue_6
                (:`Is Valid`
                  (`SoundSubsystem.PlayInGameMoleMusicSound` _returnvalue_6)
                  (`KismetSystemLibrary.PrintString` "Play Mole Music"))))
            (:`Push`
              (`/Engine/EditorBlueprintResources/StandardMacros.IsValid` _returnvalue_3
                (:`Is Valid`
                  (`SoundSubsystem.PlayInGameDeathZoneMusicSound` _returnvalue_3)
                  (`KismetSystemLibrary.PrintString` "Play Push Music"))))))))))

(fn `UserConstructionScript`)