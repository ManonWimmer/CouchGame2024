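; BP_TempPlayer is a temporary player stand-in that wanders randomly on a Y-Z plane at a fixed X.
; Tick starts a move whenever CanMove is set, clearing the flag and picking a random nearby target clamped to the Min/Max Y and Z bounds.
; The MoveToTarget timeline lerps the root component to that target, then a short delay re-enables CanMove to repeat the cycle.
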(event `CE_MoveRandomly`
  (`KismetSystemLibrary.PrintString` "move randomly")
  (set `self.CanMove` false)
  (bind _output_get (set `self.StartPosition` (`self.K2_GetActorLocation`)))
  (set `self.TargetPosition` (`KismetMathLibrary.MakeVector` 100.0 (`KismetMathLibrary.FClamp` (.y (+ _output_get (`KismetMathLibrary.MakeVector` 0.0 (`KismetMathLibrary.RandomFloatInRange` -400.0 400.0) (`KismetMathLibrary.RandomFloatInRange` -400.0 400.0)))) (`self.MinY`) (`self.MaxY`)) (`KismetMathLibrary.FClamp` (.z (+ _output_get (`KismetMathLibrary.MakeVector` 0.0 (`KismetMathLibrary.RandomFloatInRange` -400.0 400.0) (`KismetMathLibrary.RandomFloatInRange` -400.0 400.0)))) (`self.MinZ`) (`self.MaxZ`))))
  (bind (_direction _value) (`Timeline|MoveToTarget` :!via `PlayFromStart`)
    (:`Update`
      (bind (_returnvalue_x _returnvalue_y _returnvalue_z) (`KismetMathLibrary.BreakVector` (`KismetMathLibrary.VLerp` (`self.StartPosition`) (`self.TargetPosition`) _value)))
      (`SceneComponent.K2_SetWorldLocation` (`self.DefaultSceneRoot`) (`KismetMathLibrary.MakeVector` 100.0 _returnvalue_y _returnvalue_z) false false))
    (:`Finished`
      (`KismetSystemLibrary.Delay` 2.0)
      (set `self.CanMove` true))))

(event `self.ReceiveTick`
  (params (DeltaSeconds :type "Float (single-precision)"))
  (if (`self.CanMove`)
    (`self.CE_MoveRandomly`)))

(fn `UserConstructionScript`)