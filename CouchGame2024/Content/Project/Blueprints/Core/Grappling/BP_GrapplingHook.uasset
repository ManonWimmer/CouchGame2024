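; Grappling hook Blueprint that acts as an input layer for grappling and movement.
; On BeginPlay it casts player controller 0 to PC_TestGrappling, caches it and binds to its player-move event dispatcher.
; A move event passes the input vector to OnMove, and Enhanced Input IA_Grappling started, triggered and completed events call matching handlers, whose logic is defined outside these graphs.
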(event `CE_BindEventActions`
  ;[1 1 1] Bind Actions
  (add `/Game/Project/Blueprints/Core/Grappling/PC_TestGrappling.ED_OnPlayerMove` (`self.As PC Test Grappling`) (`|CreateDelegate` :!event `CE_Move`)))

(event `self.ReceiveBeginPlay`
  ;[0.2725 1 0.3156] Begin Play
  (`|ExecutionSequence`
    (:`then_0`
      (bind _aspc_test_grappling (cast `/Game/Project/Blueprints/Core/Grappling/PC_TestGrappling` (`GameplayStatics.GetPlayerController` 0)))
      (set `self.As PC Test Grappling` _aspc_test_grappling)
      (`self.CE_BindEventActions`))))

(event `CE_Move`
  (params (InputVector :type "Vector Structure"))
  ;[1 0.894 0.2377] Move
  (`self.OnMove` InputVector))

(event `EnhancedInput|/Game/Project/Input/Actions/InGame/IA_Grappling`
  (params (ActionValue :type Boolean) (ElapsedSeconds :type "Float (double-precision)") (TriggeredSeconds :type "Float (double-precision)") (InputAction :type "InputAction Object Reference" :default "/Game/Project/Input/Actions/InGame/IA_Grappling.IA_Grappling"))
  (:`Triggered`
    (`self.OnGrapplingTriggered`))
  (:`Started`
    (`self.OnGrapplingStarted`))
  (:`Completed`
    (`self.OnGrapplingCompleted`)))

(fn `UserConstructionScript`)