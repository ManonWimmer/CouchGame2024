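; Player ball Blueprint that handles the ball's gamefeel: sound, VFX, force feedback and camera shakes.
; Named events play feedback for impacts, punches, death, respawn, grappling, rails and Freeze, Slippery and Strength power-ups, using sound and camera subsystems.
; Tick scales rolling audio by velocity, swaps normal and fast trails by speed and orients the punch mesh.
; Neutral state swaps ground circles and trail assets; several VFX components keep absolute rotation.
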(event `CE_InitAbsoluteRotation`
  ;[1 1 1] Init Absolute Rotation
  (`|ExecutionSequence`
    (:`then_0`
      (set `SceneComponent.bAbsoluteRotation` true (`self.PlayerPostPhysicEffects`)))
    (:`then_1`
      (set `SceneComponent.bAbsoluteRotation` true (`self.VFX_IceBlock`)))
    (:`then_2`
      (set `SceneComponent.bAbsoluteRotation` true (`self.VFX_SlipperyActivated`)))
    (:`then_3`
      (set `SceneComponent.bAbsoluteRotation` true (`self.VFX_SlipperyActivation`)))
    (:`then_4`
      (set `SceneComponent.bAbsoluteRotation` true (`self.VFX_Impact`)))))

(event `self.PlaySetProgressStartForceEffect`
  (params (NewProgressStartForce :type "Float (single-precision)"))
  (bind _playerstartforcewidget (`self.PlayerStartForceWidget`))
  ;[0.9812 1 0.3615] Set Progress Start Force Effect
  (`/Engine/EditorBlueprintResources/StandardMacros.IsValid` _playerstartforcewidget
    (:`Is Valid`
      (`|ExecutionSequence`
        (:`then_0`
          (`/Game/Project/UMG/Player/PlayerStartForce/WBP_Player_StartForce.CE_AddToForceProgressBP` _playerstartforcewidget NewProgressStartForce))
        (:`then_1`
          (bind (_direction _impulsecolorintensity) (`Timeline|TL_ImpulseStartForceButtonEffect` :!via `PlayFromStart`)
            (:`Update`
              _)
            (:`Finished`
              _))
          (`/Game/Project/UMG/Player/PlayerStartForce/WBP_Player_StartForce.CE_SetButtonColorEffect` _playerstartforcewidget _impulsecolorintensity))))))

(event `self.ReceiveTick`
  (params (DeltaSeconds :type "Float (single-precision)"))
  ;[1 0.9353 0.4875] Tick
  (`|ExecutionSequence`
    (:`then_0`
      (`self.CE_UpdateAudioRoll`))
    (:`then_1`
      (`self.CE_updatePunchMeshRotation`))
    (:`then_2`
      (`self.CE_UpdateTrailVFX`))
    (:`then_3`
      (`self.CE_HandleGrabHandPosition`))))

(event `self.ReceiveBeginPlay`
  ;[0.3979 1 0.4708] BeginPlay
  (`|ExecutionSequence`
    (:`then_0`
      (`self.CE_InitPlayerStartForceWidget`))
    (:`then_1`
      (`AudioComponent.Stop` (`self.Audio_Wind`)))
    (:`then_2`
      (`AudioComponent.Stop` (`self.Audio_Rail`)))
    (:`then_3`
      (`self.CE_InitAbsoluteRotation`))))

(event `self.ReceiveOnSetToNeutralBall`
  ;[1 0.3404 0.9798] Neutral Switch Effects
  (`|ExecutionSequence`
    (:`then_0`
      (`SceneComponent.SetVisibility` (`self.SM_GroundCircle`) false false)
      (`SceneComponent.SetVisibility` (`self.SM_GroundCircleNeutral`) true false))
    (:`then_1`
      (`NiagaraComponent.SetAsset` (`self.VFX_TrailBall`) (`self.NeutralBasicTrail`) true)
      (`NiagaraComponent.SetAsset` (`self.VFX_TrailBallFast`) (`self.NeutralFastTrail`) true))
    (:`then_2`
      (set `self.bUseNeutral` true))))

(event `CE_SetFreezeTrail`
  (bind _freezetrail (`self.FreezeTrail`))
  (bind _vfx_trailballfast (`self.VFX_TrailBallFast`))
  (bind _vfx_trailballfast_2 (`self.VFX_TrailBallFast`))
  ;[1 0.4757 0.9041] Freeze Trail VFX
  (`|ExecutionSequence`
    (:`then_0`
      (`/Engine/EditorBlueprintResources/StandardMacros.IsValid` _vfx_trailballfast
        (:`Is Valid`
          (`/Engine/EditorBlueprintResources/StandardMacros.IsValid` _freezetrail
            (:`Is Valid`
              (`/Engine/EditorBlueprintResources/StandardMacros.IsValid` _vfx_trailballfast_2
                (:`Is Valid`
                  (`NiagaraComponent.SetAsset` _vfx_trailballfast _freezetrail true)
                  (`NiagaraComponent.SetAsset` _vfx_trailballfast_2 (`self.FreezeTrail`) true))))))))))

(event `CE_InitPlayerStartForceWidget`
  (bind _returnvalue (`WidgetComponent.GetWidget` (`self.StartForceEffectWidget`)))
  ;[0.3269 0.3191 1] Init PlayerStartForceWidget
  (`/Engine/EditorBlueprintResources/StandardMacros.IsValid` _returnvalue
    (:`Is Valid`
      (bind _aswbp_player_start_force (cast `/Game/Project/UMG/Player/PlayerStartForce/WBP_Player_StartForce` _returnvalue))
      (set `self.PlayerStartForceWidget` _aswbp_player_start_force))))

(event `CE_UnsetFreezeTrail`
  (bind _vfx_trailballfast (`self.VFX_TrailBallFast`))
  (bind _vfx_trailballfast_2 (`self.VFX_TrailBallFast`))
  (bind _vfx_trailballfast_3 (`self.VFX_TrailBallFast`))
  (bind _vfx_trailballfast_4 (`self.VFX_TrailBallFast`))
  (bind _neutralbasictrail (`self.NeutralBasicTrail`))
  (bind _neutralfasttrail (`self.NeutralFastTrail`))
  (bind _basictrail (`self.BasicTrail`))
  (bind _fasttrail (`self.FastTrail`))
  ;[1 0.4757 0.9041] Freeze Trail VFX
  (`|ExecutionSequence`
    (:`then_0`
      (if (`self.bUseNeutral`)
        (`/Engine/EditorBlueprintResources/StandardMacros.IsValid` _vfx_trailballfast_3
          (:`Is Valid`
            (`/Engine/EditorBlueprintResources/StandardMacros.IsValid` _neutralbasictrail
              (:`Is Valid`
                (`/Engine/EditorBlueprintResources/StandardMacros.IsValid` _vfx_trailballfast_4
                  (:`Is Valid`
                    (`/Engine/EditorBlueprintResources/StandardMacros.IsValid` _neutralfasttrail
                      (:`Is Valid`
                        (`NiagaraComponent.SetAsset` _vfx_trailballfast_3 _neutralfasttrail true)
                        (`NiagaraComponent.SetAsset` _vfx_trailballfast_4 _neutralbasictrail true)))))))))
        (else
          (`/Engine/EditorBlueprintResources/StandardMacros.IsValid` _vfx_trailballfast
            (:`Is Valid`
              (`/Engine/EditorBlueprintResources/StandardMacros.IsValid` _basictrail
                (:`Is Valid`
                  (`/Engine/EditorBlueprintResources/StandardMacros.IsValid` _vfx_trailballfast_2
                    (:`Is Valid`
                      (`/Engine/EditorBlueprintResources/StandardMacros.IsValid` _fasttrail
                        (:`Is Valid`
                          (`NiagaraComponent.SetAsset` _vfx_trailballfast _fasttrail true)
                          (`NiagaraComponent.SetAsset` _vfx_trailballfast_2 _basictrail true))))))))))))))

(event `CE_UpdateAudioRoll`
  (bind _audio_roll (`self.Audio_Roll`))
  (bind _audio_roll_2 (`self.Audio_Roll`))
  ;[0.4262 1 0.9701] UpdateAudioRoll
  (`/Engine/EditorBlueprintResources/StandardMacros.IsValid` _audio_roll_2
    (:`Is Valid`
      (`AudioComponent.SetVolumeMultiplier` _audio_roll_2 (`KismetMathLibrary.FInterpTo` (`AudioComponent.VolumeMultiplier` _audio_roll_2) (`KismetMathLibrary.FClamp` (/ (`KismetMathLibrary.VSize` (`self.GetVelocity`)) (`self.VelocityRef`)) 0.0 0.3) (`GameplayStatics.GetWorldDeltaSeconds`) 8.0))
      (switch `EAudioComponentPlayState` (`AudioComponent.GetPlayState` _audio_roll)
        (:`Playing`
          (if (< (`AudioComponent.VolumeMultiplier` _audio_roll) 0.02)
            (`AudioComponent.Stop` _audio_roll)))
        (:`Stopped`
          (`AudioComponent.Play` _audio_roll 0.0 :!label _label))
        (:`Paused`
          (goto _label))))))

(event `self.ReceiveOnUnsetToNeutralBall`
  ;[1 0.3404 0.9798] Neutral Switch Effects
  (`|ExecutionSequence`
    (:`then_0`
      (`SceneComponent.SetVisibility` (`self.SM_GroundCircle`) true false)
      (`SceneComponent.SetVisibility` (`self.SM_GroundCircleNeutral`) false false))
    (:`then_1`
      (`NiagaraComponent.SetAsset` (`self.VFX_TrailBall`) (`self.BasicTrail`) true)
      (`NiagaraComponent.SetAsset` (`self.VFX_TrailBallFast`) (`self.FastTrail`) true))
    (:`then_2`
      (set `self.bUseNeutral` false))))

(event `self.ReceiveOnAppearStartForceEffectWidget`
  (bind _returnvalue (subsystem `SoundSubsystem`))
  ;[1 0.4697 0.8674] Respawn Gamefeel Effects
  (`|ExecutionSequence`
    (:`then_0`
      (`KismetSystemLibrary.Delay` 1.5)
      (`/Engine/EditorBlueprintResources/StandardMacros.IsValid` _returnvalue
        (:`Is Valid`
          (`SoundSubsystem.Play321MusicSound` _returnvalue))))))

(event `self.PlayRespawnGamefeelEffectsBlueprint`
  (bind _returnvalue (subsystem `SoundSubsystem`))
  ;[1 0.4697 0.8674] Respawn Gamefeel Effects
  (`|ExecutionSequence`
    (:`then_0`
      (`/Engine/EditorBlueprintResources/StandardMacros.IsValid` _returnvalue
        (:`Is Valid`
          (`SoundSubsystem.PlayPlayerRespawnSound` _returnvalue))))))

(event `CE_UpdateTrailVFX`
  ;[1 0.3404 0.9798] Trail VFX
  (if (> (`KismetMathLibrary.VSize` (`self.GetVelocity`)) (`self.VFXTrailFastTrench`))
    (`self.CE_EnableVFXTrailFast`)
    (else
      (`self.CE_DisableVFXTrailFast`))))

(event `self.PlayImpactGamefeelEffectsBlueprint`
  (bind _returnvalue (subsystem `CameraWorldSubsystem`))
  (bind _returnvalue_2 (subsystem `SoundSubsystem`))
  (bind _vfx_impact (`self.VFX_Impact`))
  (bind _playerballcontroller (`self.PlayerBallController`))
  ;[1 0.4697 0.8674] Impact Gamefeel Effects
  (`|ExecutionSequence`
    (:`then_0`
      (`/Engine/EditorBlueprintResources/StandardMacros.IsValid` _playerballcontroller
        (:`Is Valid`
          (`PlayerController.K2_ClientPlayForceFeedback` _playerballcontroller "/Game/Project/ForceFeedbacks/FFE_Ball_Impact.FFE_Ball_Impact" "FFE_Impact" false false false))))
    (:`then_1`
      (`/Engine/EditorBlueprintResources/StandardMacros.IsValid` _returnvalue
        (:`Is Valid`
          (`CameraWorldSubsystem.PlayImpactCameraShake` _returnvalue))))
    (:`then_2`
      (`/Engine/EditorBlueprintResources/StandardMacros.IsValid` _returnvalue_2
        (:`Is Valid`
          (if (`self.GetIsImpactingNormal`)
            (`SoundSubsystem.PlayPlayerImpactsSound` _returnvalue_2)
            (else
              (`SoundSubsystem.PlayStrengthImpactSound` _returnvalue_2))))))
    (:`then_3`
      (`/Engine/EditorBlueprintResources/StandardMacros.IsValid` _vfx_impact
        (:`Is Valid`
          (`ActorComponent.Activate` _vfx_impact true))))))

(event `self.PlayDeathZoneGamefeelEffectsBlueprint`
  (bind _returnvalue (subsystem `CameraWorldSubsystem`))
  (bind _playerballcontroller (`self.PlayerBallController`))
  ;[1 0.4697 0.8674] Deathzone Gamefeel Effects
  (`|ExecutionSequence`
    (:`then_0`
      (`/Engine/EditorBlueprintResources/StandardMacros.IsValid` _playerballcontroller
        (:`Is Valid`
          (`PlayerController.K2_ClientPlayForceFeedback` _playerballcontroller "/Game/Project/ForceFeedbacks/FFE_Ball_DeathZone.FFE_Ball_DeathZone" "FFE_DeathZone" false false false))))
    (:`then_1`
      (`/Engine/EditorBlueprintResources/StandardMacros.IsValid` _returnvalue
        (:`Is Valid`
          (`CameraWorldSubsystem.PlayDeathZoneCameraShake` _returnvalue))))))

(event `self.ReceiveOnKill`
  (params (AnimDuration :type "Float (single-precision)"))
  (bind _returnvalue (subsystem `SoundSubsystem`))
  (bind _bpc_juicinessanim_scaledisappear (`self.BPC_JuicinessAnim_ScaleDisappear`))
  (bind _vfx_death (`self.VFX_Death`))
  ;[1 0.4697 0.8674] Kill Gamefeel Effects
  (`|ExecutionSequence`
    (:`then_0`
      (`/Engine/EditorBlueprintResources/StandardMacros.IsValid` _returnvalue
        (:`Is Valid`
          (`SoundSubsystem.PlayPlayerDeathSound` _returnvalue))))
    (:`then_1`
      (`/Engine/EditorBlueprintResources/StandardMacros.IsValid` _bpc_juicinessanim_scaledisappear
        (:`Is Valid`
          (`/Game/Project/Blueprints/JuicinessAnimComponents/ScaleDisappear/BPC_JuicinessAnim_ScaleDisappear.CE_PlayAnim` _bpc_juicinessanim_scaledisappear AnimDuration))))
    (:`then_2`
      (`/Engine/EditorBlueprintResources/StandardMacros.IsValid` _vfx_death
        (:`Is Valid`
          (`ActorComponent.Activate` _vfx_death true))))
    (:`then_3`
      (`|SpawnActorFromClass` "/Game/Project/Blueprints/JuicinessAnimComponents/DeathBallEffect/BP_JuicinessAnim_DeathBall.BP_JuicinessAnim_DeathBall_C" (`KismetMathLibrary.MakeTransform` (`self.K2_GetActorLocation`)) "AlwaysSpawn" "MultiplyWithRoot" null null))))

(event `CE_EnableVFXTrailFast`
  ;[1 0.3404 0.9798] Trail VFX
  (if (not (`self.bUseVFXTrailFast`))
    (set `self.bUseVFXTrailFast` true)
    (`ActorComponent.Deactivate` (`self.VFX_TrailBall`))
    (`ActorComponent.Activate` (`self.VFX_TrailBallFast`) true)))

(event `CE_DisableVFXTrailFast`
  ;[1 0.3404 0.9798] Trail VFX
  (if (`self.bUseVFXTrailFast`)
    (set `self.bUseVFXTrailFast` false)
    (`ActorComponent.Deactivate` (`self.VFX_TrailBallFast`))
    (`ActorComponent.Activate` (`self.VFX_TrailBall`) true)))

(event `self.PlayReleaseTourniquetGamefeelEffectsBlueprint`
  (bind _playerballcontroller (`self.PlayerBallController`))
  ;[1 0.4697 0.8674] Tourniquet Player Gamefeel Effects
  (`|ExecutionSequence`
    (:`then_0`
      (`/Engine/EditorBlueprintResources/StandardMacros.IsValid` _playerballcontroller
        (:`Is Valid`
          (`PlayerController.K2_ClientPlayForceFeedback` _playerballcontroller "/Game/Project/ForceFeedbacks/FFE_Ball_RelaseTourniquet.FFE_Ball_RelaseTourniquet" "FFE_ReleaseTourniquet" false false false))))))

(event `CE_TestSliperryCastEffect`
  (bind _returnvalue (subsystem `SoundSubsystem`))
  ;[1 0.4697 0.8674] Slippery Cast Gamefeel Effects
  (`|ExecutionSequence` :!label _label_2
    (:`then_0`
      (`/Engine/EditorBlueprintResources/StandardMacros.IsValid` _returnvalue
        (:`Is Valid`
          (`SoundSubsystem.PlaySlipperyCastSound` _returnvalue))))
    (:`then_1`
      (`|SpawnActorFromClass` "/Game/Project/Blueprints/PowerUps/Slippery/BP_PowerUpEffect_Slippery.BP_PowerUpEffect_Slippery_C" (`KismetMathLibrary.MakeTransform` (`self.K2_GetActorLocation`)) "AlwaysSpawn" "MultiplyWithRoot" null null))))

(event `self.PlaySlipperyCastGamefeelEffectsBlueprint`
  ;[1 0.4697 0.8674] Slippery Cast Gamefeel Effects
  (goto _label_2))

(event `self.PlayFreezeCastGamefeelEffectsBlueprint`
  (bind _returnvalue (subsystem `SoundSubsystem`))
  ;[1 0.4697 0.8674] Freeze Cast Gamefeel Effects
  (`|ExecutionSequence`
    (:`then_0`
      (`/Engine/EditorBlueprintResources/StandardMacros.IsValid` _returnvalue
        (:`Is Valid`
          (`SoundSubsystem.PlayFreezeCastSound` _returnvalue))))
    (:`then_1`
      (`|SpawnActorFromClass` "/Game/Project/Blueprints/PowerUps/Freeze/BP_PowerUpEffect_Freeze.BP_PowerUpEffect_Freeze_C" (`KismetMathLibrary.MakeTransform` (`self.K2_GetActorLocation`)) "AlwaysSpawn" "MultiplyWithRoot" null null))
    (:`then_2`
      (`self.CE_SetFreezeTrail`)
      (`KismetSystemLibrary.Delay` 2.0)
      (`self.CE_UnsetFreezeTrail`))))

(event `CE_HandleGrabHandPosition`
  ;[1 0.4697 0.8674] Grappling Grab Hand
)

(event `self.PlayPunchGamefeelEffectsBlueprint`
  (bind _returnvalue (subsystem `CameraWorldSubsystem`))
  (bind _returnvalue_2 (subsystem `SoundSubsystem`))
  (bind _playerballcontroller (`self.PlayerBallController`))
  ;[1 0.4697 0.8674] Punch Gamefeel Effects
  (`|ExecutionSequence`
    (:`then_0`
      (`/Engine/EditorBlueprintResources/StandardMacros.IsValid` _playerballcontroller
        (:`Is Valid`
          (`PlayerController.K2_ClientPlayForceFeedback` _playerballcontroller "/Game/Project/ForceFeedbacks/FFE_Ball_Punch.FFE_Ball_Punch" "FFE_Punch" false false false))))
    (:`then_1`
      (`/Engine/EditorBlueprintResources/StandardMacros.IsValid` _returnvalue
        (:`Is Valid`
          (`CameraWorldSubsystem.PlayPunchCameraShake` _returnvalue))))
    (:`then_2`
      (`/Engine/EditorBlueprintResources/StandardMacros.IsValid` _returnvalue_2
        (:`Is Valid`
          (if (`self.GetIsImpactingNormal`)
            (`SoundSubsystem.PlayPlayerPunchSound` _returnvalue_2)
            (else
              (`SoundSubsystem.PlayStrengthImpactSound` _returnvalue_2))))))))

(event `self.PlayGrapplingGrabGamefeelEffectsBlueprint`
  (bind _returnvalue (subsystem `SoundSubsystem`))
  (bind _audio_wind (`self.Audio_Wind`))
  ;[1 0.4697 0.8674] Grappling Grab Gamefeel Effects
  (`|ExecutionSequence`
    (:`then_0`
      (`/Engine/EditorBlueprintResources/StandardMacros.IsValid` _returnvalue
        (:`Is Valid`
          (`SoundSubsystem.PlayGrapplingGrabSound` _returnvalue))))
    (:`then_1`
      (`/Engine/EditorBlueprintResources/StandardMacros.IsValid` _audio_wind
        (:`Is Valid`
          (`AudioComponent.Play` _audio_wind 0.0)
          (`AudioComponent.FadeIn` _audio_wind 0.5 0.5 0.0 "Linear"))))))

(event `self.PlaySlipperyEffectGamefeelEffectsBlueprint`
  (bind _returnvalue (subsystem `SoundSubsystem`))
  ;[1 0.4697 0.8674] Slippery Effect Gamefeel Effects
  (`|ExecutionSequence`
    (:`then_0`
      (`/Engine/EditorBlueprintResources/StandardMacros.IsValid` _returnvalue
        (:`Is Valid`
          (`SoundSubsystem.PlaySlipperyEffectSound` _returnvalue))))))

(event `self.PlayGrapplingEndGamefeelEffectsBlueprint`
  (bind _audio_wind (`self.Audio_Wind`))
  ;[1 0.4697 0.8674] Grappling Grab Gamefeel Effects
  (`|ExecutionSequence`
    (:`then_0`
      (`/Engine/EditorBlueprintResources/StandardMacros.IsValid` _audio_wind
        (:`Is Valid`
          (`AudioComponent.FadeOut` _audio_wind 0.5 0.0 "Linear")
          (`AudioComponent.StopDelayed` _audio_wind 0.5))))))

(event `self.PlayPlayerFreezedGamefeelEffectsBlueprint`
  (bind _returnvalue (subsystem `SoundSubsystem`))
  (bind _vfx_iceblock (`self.VFX_IceBlock`))
  ;[1 0.4697 0.8674] Player Freezed Gamefeel Effects
  (`|ExecutionSequence`
    (:`then_0`
      (`/Engine/EditorBlueprintResources/StandardMacros.IsValid` _returnvalue
        (:`Is Valid`
          (`SoundSubsystem.PlayPlayerFreezedSound` _returnvalue))))
    (:`then_1`
      (`/Engine/EditorBlueprintResources/StandardMacros.IsValid` _vfx_iceblock
        (:`Is Valid`
          (`NiagaraComponent.ResetSystem` _vfx_iceblock)
          (`SceneComponent.SetVisibility` _vfx_iceblock true false)
          (`KismetSystemLibrary.Delay` 1.0)
          (`NiagaraComponent.SetPaused` _vfx_iceblock true))))))

(event `self.PlayPunchFailedGamefeelEffectsBlueprint`
  (bind _vfx_punchfailedzone (`self.VFX_PunchFailedZone`))
  ;[1 0.4697 0.8674] Punch Gamefeel Effects
  (`|ExecutionSequence`
    (:`then_0`
      (`/Engine/EditorBlueprintResources/StandardMacros.IsValid` _vfx_punchfailedzone
        (:`Is Valid`
          (`ActorComponent.Activate` _vfx_punchfailedzone true))))))

(event `self.PlayIsPunchedGamefeelEffectsBlueprint`
  (bind _playerballcontroller (`self.PlayerBallController`))
  ;[1 0.4697 0.8674] Punch Gamefeel Effects
  (`|ExecutionSequence`
    (:`then_0`
      (`/Engine/EditorBlueprintResources/StandardMacros.IsValid` _playerballcontroller
        (:`Is Valid`
          (`PlayerController.K2_ClientPlayForceFeedback` _playerballcontroller "/Game/Project/ForceFeedbacks/FFE_Ball_IsPunched.FFE_Ball_IsPunched" "FFE_IsPunched" false false false))))))

(event `self.PlaySlipperySlipperyDisapearGamefeelEffectsBlueprint`
  (bind _returnvalue (subsystem `SoundSubsystem`))
  ;[1 0.4697 0.8674] Slippery Disapear Gamefeel Effects
  (`|ExecutionSequence`
    (:`then_0`
      (`/Engine/EditorBlueprintResources/StandardMacros.IsValid` _returnvalue
        (:`Is Valid`
          (`SoundSubsystem.PlaySlipperySlipperyDisapearSound` _returnvalue))))))

(event `CE_TestPunchAnim`
  (bind _skm_punch (`self.SKM_Punch`))
  (bind _skm_punch_2 (`self.SKM_Punch`))
  ;[1 1 1] Punch Mesh Effect
  (set `self.bIsUpdatingPunchMeshRotation` true :!label _label_3)
  (`/Engine/EditorBlueprintResources/StandardMacros.IsValid` _skm_punch_2
    (:`Is Valid`
      (`SceneComponent.SetVisibility` _skm_punch_2 true false)
      (`SkeletalMeshComponent.PlayAnimation` _skm_punch_2 "/Game/Project/Assets/Art/07_Anim/ANIM_Punch.ANIM_Punch" false)
      (`KismetSystemLibrary.Delay` 0.7)
      (set `self.bIsUpdatingPunchMeshRotation` false)
      (`/Engine/EditorBlueprintResources/StandardMacros.IsValid` _skm_punch
        (:`Is Valid`
          (`SceneComponent.SetVisibility` _skm_punch false false))))))

(event `self.PlayPlayerUnfreezedGamefeelEffectsBlueprint`
  (bind _returnvalue (subsystem `SoundSubsystem`))
  (bind _vfx_iceblock (`self.VFX_IceBlock`))
  ;[1 0.4697 0.8674] Player UnFreezed Gamefeel Effects
  (`|ExecutionSequence`
    (:`then_0`
      (`/Engine/EditorBlueprintResources/StandardMacros.IsValid` _returnvalue
        (:`Is Valid`
          (`SoundSubsystem.PlayPlayerUnfreezeSound` _returnvalue))))
    (:`then_1`
      (`/Engine/EditorBlueprintResources/StandardMacros.IsValid` _vfx_iceblock
        (:`Is Valid`
          (`SceneComponent.SetVisibility` _vfx_iceblock false false)
          (`NiagaraComponent.SetPaused` _vfx_iceblock false))))))

(event `self.PlayPunchMeshEffect`
  (params (InTargetBall :type "PlayerBall Object Reference"))
  (bind (_returnvalue_x _returnvalue_y) (`KismetMathLibrary.BreakVector` (`self.K2_GetActorLocation` InTargetBall)))
  (bind _puncheffectroot (`self.PunchEffectRoot`))
  (bind (_returnvalue_x_2 _returnvalue_y_2 _returnvalue_z) (`KismetMathLibrary.BreakVector` (`SceneComponent.K2_GetComponentLocation` _puncheffectroot)))
  (bind (_returnvalue_location _returnvalue_rotation) (`KismetMathLibrary.BreakTransform` (`KismetAnimationLibrary.K2_LookAt` (`SceneComponent.K2_GetComponentToWorld` _puncheffectroot) (`KismetMathLibrary.MakeVector` _returnvalue_x _returnvalue_y _returnvalue_z) (`SceneComponent.GetUpVector` _puncheffectroot) false (0.0 0.0 1.0))))
  ;[1 1 1] Punch Mesh Effect
  (`|ExecutionSequence`
    (:`then_0`
      (goto _label_3))
    (:`then_1`
      (set `self.TargetPunchMeshRot` _returnvalue_rotation))))

(event `self.PlayBumpedGamefeelEffectsBlueprint`
  (bind _playerballcontroller (`self.PlayerBallController`))
  ;[1 0.4697 0.8674] Bumped Gamefeel Effects
  (`|ExecutionSequence`
    (:`then_0`
      (`/Engine/EditorBlueprintResources/StandardMacros.IsValid` _playerballcontroller
        (:`Is Valid`
          (`PlayerController.K2_ClientPlayForceFeedback` _playerballcontroller "/Game/Project/ForceFeedbacks/FFE_Ball_Bumped.FFE_Ball_Bumped" "FFE_Ball_Bumped" false false false))))))

(event `self.PlayStrengthCastGamefeelEffectsBlueprint`
  (bind _returnvalue (subsystem `SoundSubsystem`))
  (bind _returnvalue_2 (subsystem `SoundSubsystem`))
  ;[1 0.4697 0.8674] Strength Cast Gamefeel Effects
  (`|ExecutionSequence`
    (:`then_0`
      (`/Engine/EditorBlueprintResources/StandardMacros.IsValid` _returnvalue_2
        (:`Is Valid`
          (`SoundSubsystem.PlayStrengthCastSound` _returnvalue_2))))
    (:`then_1`
      (`SceneComponent.SetVisibility` (`self.SM_StrengthEffect`) true true))
    (:`then_2`
      (`/Engine/EditorBlueprintResources/StandardMacros.IsValid` _returnvalue
        (:`Is Valid`
          (`KismetSystemLibrary.Delay` 0.2)
          (`SoundSubsystem.PlayStrengthEffectSound` _returnvalue))))))

(event `self.PlayRailEnterGamefeelEffectsBlueprint`
  (bind _returnvalue (subsystem `SoundSubsystem`))
  (bind _audio_rail (`self.Audio_Rail`))
  ;[1 0.4697 0.8674] Rail Gamefeel Effects
  (`|ExecutionSequence`
    (:`then_0`
      (`/Engine/EditorBlueprintResources/StandardMacros.IsValid` _returnvalue
        (:`Is Valid`
          (`SoundSubsystem.PlayRailEnterSound` _returnvalue))))
    (:`then_1`
      (`/Engine/EditorBlueprintResources/StandardMacros.IsValid` _audio_rail
        (:`Is Valid`
          (`AudioComponent.Play` _audio_rail 0.0)
          (`AudioComponent.FadeIn` _audio_rail 0.5 1.0 0.0 "Linear"))))))

(event `self.PlayRailExitGamefeelEffectsBlueprint`
  (bind _returnvalue (subsystem `SoundSubsystem`))
  (bind _audio_rail (`self.Audio_Rail`))
  ;[1 0.4697 0.8674] Rail Gamefeel Effects
  (`|ExecutionSequence`
    (:`then_0`
      (`/Engine/EditorBlueprintResources/StandardMacros.IsValid` _returnvalue
        (:`Is Valid`
          (`SoundSubsystem.PlayRailExitSound` _returnvalue))))
    (:`then_1`
      (`/Engine/EditorBlueprintResources/StandardMacros.IsValid` _audio_rail
        (:`Is Valid`
          (`AudioComponent.FadeOut` _audio_rail 0.5 0.0 "Linear")
          (`AudioComponent.StopDelayed` _audio_rail 0.5))))))

(event `self.PlayStrengthDisapearGamefeelEffectsBlueprint`
  (bind _returnvalue (subsystem `SoundSubsystem`))
  ;[1 0.4697 0.8674] Strength Disapear Gamefeel Effects
  (`|ExecutionSequence`
    (:`then_0`
      (`/Engine/EditorBlueprintResources/StandardMacros.IsValid` _returnvalue
        (:`Is Valid`
          (`SoundSubsystem.PlayStrengthDisapearSound` _returnvalue))))
    (:`then_1`
      (`SceneComponent.SetVisibility` (`self.SM_StrengthEffect`) false true))))

(event `CE_updatePunchMeshRotation`
  (bind _puncheffectroot (`self.PunchEffectRoot`))
  (bind _puncheffectroot_2 (`self.PunchEffectRoot`))
  ;[1 1 1] Punch Mesh Effect
  (`|ExecutionSequence`
    (:`then_0`
      (`/Engine/EditorBlueprintResources/StandardMacros.IsValid` _puncheffectroot
        (:`Is Valid`
          (`SceneComponent.K2_SetWorldRotation` _puncheffectroot (`KismetMathLibrary.MakeRotator` 0.0) false false))))
    (:`then_1`
      (if (`self.bIsUpdatingPunchMeshRotation`)
        (`/Engine/EditorBlueprintResources/StandardMacros.IsValid` _puncheffectroot_2
          (:`Is Valid`
            (`SceneComponent.K2_SetWorldRotation` _puncheffectroot_2 (`self.TargetPunchMeshRot`) false false)))))))

(fn `UserConstructionScript`)