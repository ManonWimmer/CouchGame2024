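; Player controller for the player ball that handles pausing and gamepad menu navigation in both the main menu and gameplay.
; It swaps Enhanced Input mapping contexts between game and UI, and a shared UI manager records which controller paused so only it can resume.
; Stick input with a repeat delay, confirm and back are forwarded to pause, settings, credits or winner widgets on whichever HUD is active.
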(event `CE_SwitchToIMC_UI`
  (bind _returnvalue (subsystem `EnhancedInputLocalPlayerSubsystem`))
  (`KismetSystemLibrary.PrintString` "switch to ui")
  (`/Engine/EditorBlueprintResources/StandardMacros.IsValid` _returnvalue
    (:`Is Valid`
      (`EnhancedInputSubsystemInterface.RemoveMappingContext` _returnvalue "/Game/Project/Input/IMCs/Gamepads/IMC_gamepads_InGame.IMC_gamepads_InGame" (struct))
      (`EnhancedInputSubsystemInterface.AddMappingContext` _returnvalue "/Game/Project/Input/IMCs/IMC_UI.IMC_UI" 0 (struct))
      (`WidgetBlueprintLibrary.SetInputMode_GameAndUIEx` self null)
      (`WidgetBlueprintLibrary.SetFocusToGameViewport`))))

(event `CE_SwitchToIMC_Game`
  (bind _returnvalue (subsystem `EnhancedInputLocalPlayerSubsystem`))
  (`/Engine/EditorBlueprintResources/StandardMacros.IsValid` _returnvalue
    (:`Is Valid`
      (`EnhancedInputSubsystemInterface.RemoveMappingContext` _returnvalue "/Game/Project/Input/IMCs/IMC_UI.IMC_UI" (struct))
      (`EnhancedInputSubsystemInterface.AddMappingContext` _returnvalue "/Game/Project/Input/IMCs/Gamepads/IMC_gamepads_InGame.IMC_gamepads_InGame" 0 (struct))
      (`WidgetBlueprintLibrary.SetInputMode_GameOnly` self))))

(event `EnhancedInput|/Game/Project/Input/Actions/UI/IA_Pause`
  (params (ActionValue :type Boolean) (ElapsedSeconds :type "Float (double-precision)") (TriggeredSeconds :type "Float (double-precision)") (InputAction :type "InputAction Object Reference" :default "/Game/Project/Input/Actions/UI/IA_Pause.IA_Pause"))
  (:`Started`
    (`self.CE_PauseTriggered`)))

(event `CE_PauseTriggered`
  ;[0.162 0.9216 1] Pause Triggered
  (`KismetSystemLibrary.PrintString` "PAUSE")
  (if (`GameplayStatics.IsGamePaused`)
    (`self.CE_CheckCanClosePause`)
    (if (`self.CanClosePause`)
      (`GameplayStatics.SetGamePaused` false)
      (`self.CE_HidePauseWidget`)
      (`self.CE_SwitchToIMC_Game`))
    (else
      (`self.CE_CheckCanOpenPause`)
      (if (`self.CanOpenPause`)
        (`GameplayStatics.SetGamePaused` true)
        (`self.CE_ShowPauseWidget`)
        (`self.CE_SwitchToIMC_UI`)
        (set `/Game/Project/Blueprints/UI/BP_UIManager.PauseController` self (`self.UIManager`))))))

(event `self.ReceiveBeginPlay`
  (`self.CE_GetUIManager`)
  (`self.CE_GetHUDs`)
  (`KismetSystemLibrary.PrintString` "Player Controller" true true (struct :`R` 1.0 :`G` 0.54931 :`B` 0.453276 :`A` 1.0) 10.0))

(event `CE_GetHUDs`
  (bind _returnvalue (`self.GetHUD` (`GameplayStatics.GetPlayerController` 0)))
  (bind _ashud_in_game (cast `/Game/Project/Blueprints/Core/HUDs/HUD_InGame` _returnvalue)
    (:`then`
      (set `self.HUD_Game` _ashud_in_game))
    (:`CastFailed`
      (bind _ashud_main_menu (cast `/Game/Project/Blueprints/Core/HUDs/HUD_MainMenu` _returnvalue))
      (set `self.HUD_MainMenu` _ashud_main_menu)
      (set `self.InMainMenu` true))))

(event `CE_HidePauseWidget`
  ;[0.162 0.9216 1] Hide Pause
  (if (`self.InMainMenu`)
    (`/Game/Project/UMG/WBP_Pause_Menu.CE_Resume` (`/Game/Project/Blueprints/Core/HUDs/HUD_MainMenu.PauseMenu` (`self.HUD_MainMenu`)))
    (else
      (`/Game/Project/UMG/WBP_Pause_Menu.CE_Resume` (`/Game/Project/Blueprints/Core/HUDs/HUD_InGame.PauseMenu` (`self.HUD_Game`))))))

(event `EnhancedInput|/Game/Project/Input/Actions/UI/IA_MoveUI`
  (params (ActionValue :type "Vector2D Structure") (ElapsedSeconds :type "Float (double-precision)") (TriggeredSeconds :type "Float (double-precision)") (InputAction :type "InputAction Object Reference" :default "/Game/Project/Input/Actions/UI/IA_MoveUI.IA_MoveUI"))
  (:`Triggered`
    (`|ExecutionSequence`
      (:`then_0`
        ;[1 1 1] Up
        (if (> ActionValue_Y 0.7)
          (if (or (== (`self.LastMoveTime`) 0.0) (> (- ElapsedSeconds (`self.LastMoveTime`)) (`self.MoveDelay`)))
            (set `self.LastMoveTime` ElapsedSeconds)
            (`KismetSystemLibrary.PrintString` "UP")
            (`self.CE_SelectPauseButton` "NewEnumerator0"))))
      (:`then_1`
        ;[1 1 1] Down
        (if (< ActionValue_Y -0.7)
          (if (or (== (`self.LastMoveTime`) 0.0) (> (- ElapsedSeconds (`self.LastMoveTime`)) (`self.MoveDelay`)))
            (set `self.LastMoveTime` ElapsedSeconds)
            (`KismetSystemLibrary.PrintString` "DOWN")
            (`self.CE_SelectPauseButton` "NewEnumerator1"))))
      (:`then_2`
        ;[1 1 1] Right
        (if (> ActionValue_X 0.7)
          (if (or (== (`self.LastMoveTime`) 0.0) (> (- ElapsedSeconds (`self.LastMoveTime`)) (`self.MoveDelay`)))
            (set `self.LastMoveTime` ElapsedSeconds)
            (`KismetSystemLibrary.PrintString` "RIGHT")
            (`self.CE_SelectPauseButton` "NewEnumerator3"))))
      (:`then_3`
        ;[1 1 1] Left
        (if (< ActionValue_X -0.7)
          (if (or (== (`self.LastMoveTime`) 0.0) (> (- ElapsedSeconds (`self.LastMoveTime`)) (`self.MoveDelay`)))
            (set `self.LastMoveTime` ElapsedSeconds)
            (`KismetSystemLibrary.PrintString` "LEFT")
            (`self.CE_SelectPauseButton` "NewEnumerator2"))))))
  (:`Started`
    (set `self.StartMoveTime` ElapsedSeconds)
    (set `self.LastMoveTime` 0.0)))

(event `CE_ShowSettingsWidget`
  ;[1 0.6867 0.2664] Show Settings
  (if (`self.InMainMenu`)
    (`Widget.SetVisibility` (`/Game/Project/Blueprints/Core/HUDs/HUD_MainMenu.SettingsMenu` (`self.HUD_MainMenu`)) "Visible")
    (else
      (`Widget.SetVisibility` (`/Game/Project/Blueprints/Core/HUDs/HUD_InGame.SettingsMenu` (`self.HUD_Game`)) "Visible"))))

(event `CE_ShowPauseWidget`
  ;[0.162 0.9216 1] Show Pause
  (if (`self.InMainMenu`)
    (`Widget.SetVisibility` (`/Game/Project/Blueprints/Core/HUDs/HUD_MainMenu.PauseMenu` (`self.HUD_MainMenu`)) "Visible")
    (else
      (`Widget.SetVisibility` (`/Game/Project/Blueprints/Core/HUDs/HUD_InGame.PauseMenu` (`self.HUD_Game`)) "Visible"))))

(event `CE_HideSettingsWidget`
  ;[1 0.6867 0.2664] Hide Settings
  (if (`self.InMainMenu`)
    (`/Game/Project/UMG/WBP_Settings_Menu.CE_CloseSettings` (`/Game/Project/Blueprints/Core/HUDs/HUD_MainMenu.SettingsMenu` (`self.HUD_MainMenu`)))
    (else
      (`/Game/Project/UMG/WBP_Settings_Menu.CE_CloseSettings` (`/Game/Project/Blueprints/Core/HUDs/HUD_InGame.SettingsMenu` (`self.HUD_Game`))))))

(event `CE_SelectPauseButton`
  (params (Direction :type "/Game/Project/Input/E_DirectionUI Enum" :default "NewEnumerator0"))
  ;[0.162 0.9216 1] Select Pause Button
  (if (`self.InMainMenu`)
    (`/Game/Project/UMG/WBP_Pause_Menu.CE_SelectPauseButtonGamepad` (`/Game/Project/Blueprints/Core/HUDs/HUD_MainMenu.PauseMenu` (`self.HUD_MainMenu`)) Direction)
    (else
      (`/Game/Project/UMG/WBP_Pause_Menu.CE_SelectPauseButtonGamepad` (`/Game/Project/Blueprints/Core/HUDs/HUD_InGame.PauseMenu` (`self.HUD_Game`)) Direction))))

(event `CE_PlayFadeOutPause`
  ;[0.162 0.9216 1] Play Fade Out Pause
  (if (`self.InMainMenu`)
    (`/Game/Project/UMG/WBP_Pause_Menu.CE_FadeOutAnimationForSettings` (`/Game/Project/Blueprints/Core/HUDs/HUD_MainMenu.PauseMenu` (`self.HUD_MainMenu`)))
    (else
      (`/Game/Project/UMG/WBP_Pause_Menu.CE_FadeOutAnimationForSettings` (`/Game/Project/Blueprints/Core/HUDs/HUD_InGame.PauseMenu` (`self.HUD_Game`))))))

(event `EnhancedInput|/Game/Project/Input/Actions/UI/IA_ConfirmUI`
  (params (ActionValue :type Boolean) (ElapsedSeconds :type "Float (double-precision)") (TriggeredSeconds :type "Float (double-precision)") (InputAction :type "InputAction Object Reference" :default "/Game/Project/Input/Actions/UI/IA_ConfirmUI.IA_ConfirmUI"))
  (bind _pausemenu (`/Game/Project/Blueprints/Core/HUDs/HUD_MainMenu.PauseMenu` (`self.HUD_MainMenu`)))
  (bind _pausemenu_2 (`/Game/Project/Blueprints/Core/HUDs/HUD_InGame.PauseMenu` (`self.HUD_Game`)))
  (bind _winnerwidget (`/Game/Project/Blueprints/Core/HUDs/HUD_InGame.WinnerWidget` (`self.HUD_Game`)))
  (bind _creditsmenu (`/Game/Project/Blueprints/Core/HUDs/HUD_InGame.CreditsMenu` (`self.HUD_Game`)))
  (bind _creditsmenu_2 (`/Game/Project/Blueprints/Core/HUDs/HUD_MainMenu.CreditsMenu` (`self.HUD_MainMenu`)))
  ;[1 0.4969 0.7454] Confirm UI
  (:`Started`
    (if (`self.InMainMenu`)
      (if (`Widget.IsVisible` _creditsmenu_2)
        (`/Game/Project/UMG/WBP_Credits.CE_BackToMenu` _creditsmenu_2)
        (elif (`Widget.IsVisible` _pausemenu)
          (`/Game/Project/UMG/WBP_Pause_Menu.CE_ConfirmPauseButton` _pausemenu)))
      (elif (`Widget.IsVisible` _creditsmenu)
        (`/Game/Project/UMG/WBP_Credits.CE_BackToMenu` _creditsmenu)
        (elif (`Widget.IsVisible` _pausemenu_2)
          (`/Game/Project/UMG/WBP_Pause_Menu.CE_ConfirmPauseButton` _pausemenu_2)
          (elif (`Widget.IsVisible` _winnerwidget)
            (`/Game/Project/UMG/WBP_Winner.CE_WinnerBackToMenu` _winnerwidget)))))))

(event `CE_PlayFadeInSettings`
  ;[1 0.6867 0.2664] Play Fade In Settings
  (if (`self.InMainMenu`)
    (`/Game/Project/UMG/WBP_Settings_Menu.CE_FadeInAnimation` (`/Game/Project/Blueprints/Core/HUDs/HUD_MainMenu.SettingsMenu` (`self.HUD_MainMenu`)))
    (else
      (`/Game/Project/UMG/WBP_Settings_Menu.CE_FadeInAnimation` (`/Game/Project/Blueprints/Core/HUDs/HUD_InGame.SettingsMenu` (`self.HUD_Game`))))))

(event `EnhancedInput|/Game/Project/Input/Actions/UI/IA_BackUI`
  (params (ActionValue :type Boolean) (ElapsedSeconds :type "Float (double-precision)") (TriggeredSeconds :type "Float (double-precision)") (InputAction :type "InputAction Object Reference" :default "/Game/Project/Input/Actions/UI/IA_BackUI.IA_BackUI"))
  (bind _creditsmenu (`/Game/Project/Blueprints/Core/HUDs/HUD_InGame.CreditsMenu` (`self.HUD_Game`)))
  (bind _pausemenu (`/Game/Project/Blueprints/Core/HUDs/HUD_MainMenu.PauseMenu` (`self.HUD_MainMenu`)))
  (bind _pausemenu_2 (`/Game/Project/Blueprints/Core/HUDs/HUD_InGame.PauseMenu` (`self.HUD_Game`)))
  (bind _creditsmenu_2 (`/Game/Project/Blueprints/Core/HUDs/HUD_MainMenu.CreditsMenu` (`self.HUD_MainMenu`)))
  ;[1 0.4969 0.7454] Back UI
  (:`Started`
    (if (`self.InMainMenu`)
      (if (`Widget.IsVisible` _creditsmenu_2)
        (`/Game/Project/UMG/WBP_Credits.CE_BackToMenu` _creditsmenu_2)
        (elif (`Widget.IsVisible` _pausemenu)
          (`/Game/Project/UMG/WBP_Pause_Menu.CE_BackPauseButton` _pausemenu)))
      (elif (`Widget.IsVisible` _creditsmenu)
        (`/Game/Project/UMG/WBP_Credits.CE_BackToMenu` _creditsmenu)
        (elif (`Widget.IsVisible` _pausemenu_2)
          (`/Game/Project/UMG/WBP_Pause_Menu.CE_BackPauseButton` _pausemenu_2))))))

(event `CE_PlayFadeOutSettings`
  ;[1 0.6867 0.2664] Play Fade Out Settings
  (if (`self.InMainMenu`)
    (`/Game/Project/UMG/WBP_Settings_Menu.CE_FadeOutAnimation` (`/Game/Project/Blueprints/Core/HUDs/HUD_MainMenu.SettingsMenu` (`self.HUD_MainMenu`)))
    (else
      (`/Game/Project/UMG/WBP_Settings_Menu.CE_FadeOutAnimation` (`/Game/Project/Blueprints/Core/HUDs/HUD_InGame.SettingsMenu` (`self.HUD_Game`))))))

(event `CE_SelectSettingsButtonGamepad`
  (params (Direction :type "/Game/Project/Input/E_DirectionUI Enum" :default "NewEnumerator0"))
  ;[1 0.6867 0.2664] Select Settings Button Gamepad
  (if (`self.InMainMenu`)
    (`/Game/Project/UMG/WBP_Settings_Menu.CE_SelectSettingsButtonGamepad` (`/Game/Project/Blueprints/Core/HUDs/HUD_MainMenu.SettingsMenu` (`self.HUD_MainMenu`)) Direction)
    (else
      (`/Game/Project/UMG/WBP_Settings_Menu.CE_SelectSettingsButtonGamepad` (`/Game/Project/Blueprints/Core/HUDs/HUD_InGame.SettingsMenu` (`self.HUD_Game`)) Direction))))

(event `CE_GetUIManager`
  (bind _returnvalue (`GameplayStatics.GetActorOfClass` "/Game/Project/Blueprints/UI/BP_UIManager.BP_UIManager_C"))
  (set `self.UIManager` _returnvalue))

(event `CE_CreditsTriggered`
  (bind _creditsmenu (`/Game/Project/Blueprints/Core/HUDs/HUD_InGame.CreditsMenu` (`self.HUD_Game`)))
  (bind _creditsmenu_2 (`/Game/Project/Blueprints/Core/HUDs/HUD_MainMenu.CreditsMenu` (`self.HUD_MainMenu`)))
  ;[0.4222 1 0.4605] Credits Triggered
  (if (`self.InMainMenu`)
    (if (`Widget.IsVisible` _creditsmenu_2)
      (`/Game/Project/UMG/WBP_Credits.CE_BackToMenu` _creditsmenu_2)
      (else
        (`self.CE_PlayFadeOutSettings`)
        (`KismetSystemLibrary.Delay` 0.5)
        (`Widget.SetVisibility` _creditsmenu_2 "Visible")))
    (elif (`Widget.IsVisible` _creditsmenu)
      (`/Game/Project/UMG/WBP_Credits.CE_BackToMenu` _creditsmenu)
      (else
        (`self.CE_PlayFadeOutSettings`)
        (`KismetSystemLibrary.Delay` 0.5)
        (`Widget.SetVisibility` _creditsmenu "Visible")))))

(event `CE_CheckCanOpenPause`
  (bind _hud_game (`self.HUD_Game`))
  ;[0.162 0.9216 1] Check Can Open Pause
  (set `self.CanOpenPause` true)
  (if (`self.InMainMenu`)
    _
    (elif (or (`Widget.IsVisible` (`/Game/Project/Blueprints/Core/HUDs/HUD_InGame.NextRoundWidget` _hud_game)) (`Widget.IsVisible` (`/Game/Project/Blueprints/Core/HUDs/HUD_InGame.WinnerWidget` _hud_game)))
      (set `self.CanOpenPause` false))))

(event `CE_CheckCanClosePause`
  ;[0.162 0.9216 1] Check Can Close Pause
  (set `self.CanClosePause` (== (`/Game/Project/Blueprints/UI/BP_UIManager.PauseController` (`self.UIManager`)) self)))

(fn `UserConstructionScript`)