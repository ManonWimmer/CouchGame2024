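; BP_PowerUpEffect_Freeze is the visual effect actor for the area-of-effect Freeze power-up.
; On BeginPlay, if its skeletal mesh is valid, it plays a one-shot spawn animation, then switches to a looping rotate animation after a short delay.
; After a further delay, a vector tween shrinks the actor's scale, and the actor destroys itself when the tween completes.
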(event `self.ReceiveBeginPlay`
  (bind _skm_freezeeffect (`self.SKM_FreezeEffect`))
  ;[0.4211 1 0.4236] Begin Play
  (`/Engine/EditorBlueprintResources/StandardMacros.IsValid` _skm_freezeeffect
    (:`Is Valid`
      (`SkeletalMeshComponent.PlayAnimation` _skm_freezeeffect "/Game/Project/Assets/Art/07_Anim/freeze_AOE/SM_PowerUp_Freeze_AOE_Spawn_Anim.SM_PowerUp_Freeze_AOE_Spawn_Anim" false)
      (`KismetSystemLibrary.Delay` 0.5)
      (`SkeletalMeshComponent.PlayAnimation` (`self.SKM_FreezeEffect`) "/Game/Project/Assets/Art/07_Anim/freeze_AOE/SM_PowerUp_Freeze_AOE_Rotate_Anim.SM_PowerUp_Freeze_AOE_Rotate_Anim" true)
      (`KismetSystemLibrary.Delay` 1.0)
      (bind (_asynctaskproxy _value) (`FCTweenBPActionVector.TweenVector` (`self.GetActorScale3D`) (0.1 0.1 0.1))
        (:`ApplyEasing`
          (`self.SetActorScale3D` _value))
        (:`OnComplete`
          (`self.K2_DestroyActor`))))))

(fn `UserConstructionScript`)