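; BP_PowerUp_Slippery is the Slippery power-up Blueprint, and this graph handles only its appear animation.
; On BeginPlay it calls CE_InitAnims, which passes the scale-appear duration from PowerUpAnimData to the BPCJuicinessAnimScaleAppear component.
; It then starts that component's animation, with validity checks guarding both steps.
; The slippery effect itself is not implemented in these graphs, and the construction script is empty.
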(event `CE_InitAnims`
  (bind _bpc_juicinessanim_scaleappear (`self.BPC_JuicinessAnim_ScaleAppear`))
  ;[1 1 1] Init Anims
  (`/Engine/EditorBlueprintResources/StandardMacros.IsValid` null
    (:`Is Valid`
      (`|ExecutionSequence`
        (:`then_0`
          (`/Engine/EditorBlueprintResources/StandardMacros.IsValid` _bpc_juicinessanim_scaleappear
            (:`Is Valid`
              (`/Game/Project/Blueprints/JuicinessAnimComponents/ScaleAppear/BPC_JuicinessAnim_ScaleAppear.CE_InitAnim` _bpc_juicinessanim_scaleappear (`JuicinessAnimData.PowerUpScaleAppearDuration` (`self.PowerUpAnimData`))))))))))

(event `self.ReceiveBeginPlay`
  (bind _bpc_juicinessanim_scaleappear (`self.BPC_JuicinessAnim_ScaleAppear`))
  ;[0.4048 1 0.562] Begin Play
  (`|ExecutionSequence`
    (:`then_0`
      (`self.CE_InitAnims`))
    (:`then_1`
      (`/Engine/EditorBlueprintResources/StandardMacros.IsValid` _bpc_juicinessanim_scaleappear
        (:`Is Valid`
          (`/Game/Project/Blueprints/JuicinessAnimComponents/ScaleAppear/BPC_JuicinessAnim_ScaleAppear.CE_StartAnim` _bpc_juicinessanim_scaleappear))))))

(fn `UserConstructionScript`)