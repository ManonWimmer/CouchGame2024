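; Actor component that adds a juicy yoyo effect by tweening its owner's pitch between negative and positive amplitude.
; CE_InitAnim overrides duration when non-zero, but a non-zero amplitude argument sets YoyoAmplitude to zero instead of storing it.
; CE_StartAnim runs a TweenFloat that writes its value as the owner's absolute pitch on each easing update.
; The starting rotation is cached in BaseRot but not used.
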(event `CE_InitAnim`
  (params (AnimDuration :type "Float (double-precision)") (YoyoAmplitude :type "Float (double-precision)"))
  ;[1 1 1] Init Anim
  (`|ExecutionSequence`
    (:`then_0`
      (if (!= AnimDuration 0.0)
        (set `self.AnimDuration` AnimDuration)))
    (:`then_1`
      (if (!= YoyoAmplitude 0.0)
        (set `self.YoyoAmplitude` 0.0)))))

(event `CE_StartAnim`
  (bind _returnvalue (`self.GetOwner`))
  (bind _returnvalue_2 (`self.GetOwner`))
  (bind _yoyoamplitude (`self.YoyoAmplitude`))
  ;[0.3988 1 0.5632] Start Anim
  (`|ExecutionSequence`
    (:`then_0`
      (`/Engine/EditorBlueprintResources/StandardMacros.IsValid` _returnvalue_2
        (:`Is Valid`
          (set `self.BaseRot` (`Actor.K2_GetActorRotation` _returnvalue_2)))))
    (:`then_1`
      (bind (_asynctaskproxy _value) (`FCTweenBPActionFloat.TweenFloat` (* _yoyoamplitude -1.0) _yoyoamplitude (`self.AnimDuration`) "InOutQuad" 0.0 0.0 0.0 0 0.0 true)
        (:`ApplyEasing`
          (`/Engine/EditorBlueprintResources/StandardMacros.IsValid` _returnvalue
            (:`Is Valid`
              (`Actor.K2_SetActorRotation` _returnvalue (`KismetMathLibrary.MakeRotator` 0.0 _value) false))))))))