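; Actor component that plays a juicy "scale appear" animation on its owning actor.
; Starting it captures the owner's current scale as the target, then tweens from a start scale to it with elastic ease-out, applying each value to the actor.
; An init event takes a non-zero duration, and the stored async tween task lets a stop event cancel the animation.
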(event `CE_InitAnim`
  (params (AnimDuration :type "Float (double-precision)"))
  ;[1 1 1] Init Anim
  (if (!= AnimDuration 0.0)
    (set `self.AnimDuration` AnimDuration)))

(event `CE_StopAnim`
  (bind _asyncscaleappear (`self.AsyncScaleAppear`))
  ;[1 1 1] Stop Anim
  (`/Engine/EditorBlueprintResources/StandardMacros.IsValid` _asyncscaleappear
    (:`Is Valid`
      (`FCTweenBPAction.Stop` _asyncscaleappear))))

(event `CE_ScaleAppear`
  ;[1 0.3359 0.9045] Scale Appear Anim
  (`/Engine/EditorBlueprintResources/StandardMacros.IsValid` (`self.GetOwner`)
    (:`Is Valid`
      (bind (_asynctaskproxy _value) (`FCTweenBPActionVector.TweenVector` (`self.StartScale`) (`self.TargetScale`) (`self.AnimDuration`) "OutElastic")
        (:`then`
          (set `self.AsyncScaleAppear` _asynctaskproxy))
        (:`ApplyEasing`
          (`Actor.SetActorScale3D` (`self.GetOwner`) _value))))))

(event `CE_StartAnim`
  (bind _returnvalue (`self.GetOwner`))
  ;[0.8338 1 0.3009] Start Anim
  (`/Engine/EditorBlueprintResources/StandardMacros.IsValid` _returnvalue
    (:`Is Valid`
      (set `self.TargetScale` (`Actor.GetActorScale3D` _returnvalue))
      (`self.CE_ScaleAppear`))))