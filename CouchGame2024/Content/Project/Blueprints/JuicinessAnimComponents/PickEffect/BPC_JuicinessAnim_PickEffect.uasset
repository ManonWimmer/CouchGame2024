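; Juiciness component that animates its owning actor when picked, apparently a duck.
; CE_PickAnim starts three parallel tweens on the owner: an eased yaw spin toward 400 degrees wrapped at 360, an eased upward move, and a scale change divided by TargetScaleDivider.
; Spin and scale share RotateDuration, while the rise uses JumpDuration.
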(event `CE_PickAnim`
  (bind _returnvalue (`self.GetOwner`))
  (bind (_returnvalue_roll _returnvalue_pitch _returnvalue_yaw) (`KismetMathLibrary.BreakRotator` (`Actor.K2_GetActorRotation` _returnvalue)))
  (bind _returnvalue_2 (`Actor.K2_GetActorLocation` (`self.GetOwner`)))
  (bind _returnvalue_3 (`Actor.GetActorScale3D` (`self.GetOwner`)))
  ;[1 0.5051 0.8411] Pick Duck
  (`/Engine/EditorBlueprintResources/StandardMacros.IsValid` _returnvalue
    (:`Is Valid`
      (`|ExecutionSequence`
        (:`then_0`
          (bind (_asynctaskproxy _value) (`FCTweenBPActionFloat.TweenFloat` _returnvalue_yaw 400.0 (`self.RotateDuration`) "InQuad")
            (:`ApplyEasing`
              (`Actor.K2_SetActorRotation` (`self.GetOwner`) (`KismetMathLibrary.MakeRotator` 0.0 0.0 (mod _value 360.0)) false))))
        (:`then_1`
          (bind (_asynctaskproxy_2 _value_2) (`FCTweenBPActionVector.TweenVector` _returnvalue_2 (+ _returnvalue_2 (0.0 0.0 100.0)) (`self.JumpDuration`) "OutQuad")
            (:`ApplyEasing`
              (`Actor.K2_SetActorLocation` (`self.GetOwner`) _value_2 false false))))
        (:`then_2`
          (bind (_asynctaskproxy_3 _value_3) (`FCTweenBPActionVector.TweenVector` _returnvalue_3 (/ _returnvalue_3 (`self.TargetScaleDivider`)) (`self.RotateDuration`))
            (:`ApplyEasing`
              (`Actor.SetActorScale3D` (`self.GetOwner`) _value_3))))))))