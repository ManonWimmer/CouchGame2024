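; Juiciness animation component that spins its owning actor around the yaw axis, named as an infinite rotation.
; On BeginPlay it zeroes the owner's rotation, then starts a linear float tween toward a full turn over RotateDuration.
; A random start delay, capped by RandomDelayMax, varies timing between instances.
; Each easing update sets the owner's yaw, and the stored async task lets CE_StopAnim halt the spin.
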(event `CE_StopAnim`
  (bind _asyncrotate (`self.AsyncRotate`))
  ;[1 1 1] Stop Anim
  (`/Engine/EditorBlueprintResources/StandardMacros.IsValid` _asyncrotate
    (:`Is Valid`
      (`FCTweenBPAction.Stop` _asyncrotate))))

(event `CE_RotateAnim`
  ;[1 0.3359 0.9045] Rotate Anim
  (`/Engine/EditorBlueprintResources/StandardMacros.IsValid` (`self.GetOwner`)
    (:`Is Valid`
      (bind (_asynctaskproxy _value) (`FCTweenBPActionFloat.TweenFloat` 0.0 360.0 (`self.RotateDuration`) "Linear" 0.0 0.0 (`KismetMathLibrary.RandomFloatInRange` 0.0 (`self.RandomDelayMax`)) -1)
        (:`then`
          (set `self.AsyncRotate` _asynctaskproxy))
        (:`ApplyEasing`
          (`Actor.K2_SetActorRotation` (`self.GetOwner`) (`KismetMathLibrary.MakeRotator` 0.0 0.0 _value) false))))))

(event `self.ReceiveBeginPlay`
  (bind _returnvalue (`self.GetOwner`))
  ;[0.3672 1 0.3979] BeginPlay
  (`|ExecutionSequence`
    (:`then_0`
      (`/Engine/EditorBlueprintResources/StandardMacros.IsValid` _returnvalue
        (:`Is Valid`
          (`Actor.K2_SetActorRotation` :`self` _returnvalue))))
    (:`then_1`
      (`self.CE_RotateAnim`))))