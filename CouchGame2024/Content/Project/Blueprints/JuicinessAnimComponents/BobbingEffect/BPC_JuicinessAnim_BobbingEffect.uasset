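; Actor component that adds a juicy bobbing animation to its owner.
; On BeginPlay it starts an async vector tween from the owner's location to a vertical offset, applying each eased value as the actor's location.
; A random start delay, up to a configurable maximum, can keep multiple instances out of sync.
; The stored tween task lets a stop event cancel the animation.
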(event `CE_StopAnim`
  (bind _asyncbobbing (`self.AsyncBobbing`))
  ;[1 1 1] Stop Anim
  (`/Engine/EditorBlueprintResources/StandardMacros.IsValid` _asyncbobbing
    (:`Is Valid`
      (`FCTweenBPAction.Stop` _asyncbobbing))))

(event `CE_BobbingAnim`
  (bind _returnvalue (`self.GetOwner`))
  (bind _returnvalue_2 (`Actor.K2_GetActorLocation` _returnvalue))
  ;[1 0.3359 0.9045] Bobbing Anim
  (`/Engine/EditorBlueprintResources/StandardMacros.IsValid` _returnvalue
    (:`Is Valid`
      (bind (_asynctaskproxy _value) (`FCTweenBPActionVector.TweenVector` _returnvalue_2 (+ _returnvalue_2 (`KismetMathLibrary.MakeVector` 0.0 0.0 (`self.BobbingOffset`))) (`self.BobbingDuration`) "InOutQuad" 0.0 0.0 (`KismetMathLibrary.RandomFloatInRange` 0.0 (`self.RandomDelayMax`)) -1 0.0 true)
        (:`then`
          (set `self.AsyncBobbing` _asynctaskproxy))
        (:`ApplyEasing`
          (`Actor.K2_SetActorLocation` (`self.GetOwner`) _value false false))))))

(event `self.ReceiveBeginPlay`
  ;[0.3672 1 0.3979] BeginPlay
  (`|ExecutionSequence`
    (:`then_0`
      (`self.CE_BobbingAnim`))))