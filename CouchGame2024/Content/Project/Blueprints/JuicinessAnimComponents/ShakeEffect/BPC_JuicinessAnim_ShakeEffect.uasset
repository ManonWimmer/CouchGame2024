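; Juiciness animation component that shakes its owning actor horizontally when CE_StartShake is called.
; BeginPlay caches the owner's location as the shake origin.
; A TweenFloat serves as the update driver: each easing update moves the owner to that origin plus random X and Y offsets between zero and Intensity, keeping current Z.
; Offsets are positive only, and no step restores the original location afterwards.
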(event `self.ReceiveBeginPlay`
  (bind _returnvalue (`self.GetOwner`))
  ;[0.4713 1 0.5044] Begin Play
  (`/Engine/EditorBlueprintResources/StandardMacros.IsValid` _returnvalue
    (:`Is Valid`
      (set `self.StartLocation` (`Actor.K2_GetActorLocation` _returnvalue)))))

(event `CE_StartShake`
  (bind _returnvalue (`self.GetOwner`))
  (bind (_startlocation_x _startlocation_y) (`KismetMathLibrary.BreakVector` (`self.StartLocation`)))
  (bind (_returnvalue_x _returnvalue_y _returnvalue_z) (`KismetMathLibrary.BreakVector` (`Actor.K2_GetActorLocation` _returnvalue)))
  ;[1 0.5394 0.9612] Start Shake
  (`FCTweenBPActionFloat.TweenFloat` 0.0
    (:`ApplyEasing`
      (`/Engine/EditorBlueprintResources/StandardMacros.IsValid` _returnvalue
        (:`Is Valid`
          (`Actor.K2_SetActorLocation` _returnvalue (`KismetMathLibrary.MakeVector` (+ _startlocation_x (`KismetMathLibrary.RandomFloatInRange` 0.0 (`self.Intensity`))) (+ _startlocation_y (`KismetMathLibrary.RandomFloatInRange` 0.0 (`self.Intensity`))) _returnvalue_z) false false))))))