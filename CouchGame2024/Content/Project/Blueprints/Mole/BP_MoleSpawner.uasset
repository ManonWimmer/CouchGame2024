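; BP_MoleSpawner is a mole spawn point that handles the mud effect shown when a mole appears or leaves.
; On spawn it reveals and restarts the VFXMud particle component, then uses the TL_DelayBeforePause timeline as a delay before pausing the effect.
; Despawn and forced-destroy events both simply hide the mud.
; The graph holds only these visual responses, with no spawning logic of its own.
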(event `self.ReceiveOnSpawnMole`
  (bind _vfx_mud (`self.VFX_Mud`))
  (bind _vfx_mud_2 (`self.VFX_Mud`))
  ;[1 0.4983 0.9027] On Spawn Mole
  (`|ExecutionSequence`
    (:`then_0`
      (`/Engine/EditorBlueprintResources/StandardMacros.IsValid` _vfx_mud_2
        (:`Is Valid`
          (`SceneComponent.SetVisibility` _vfx_mud_2 true false)
          (`ActorComponent.Activate` _vfx_mud_2 true)
          (`NiagaraComponent.ResetSystem` _vfx_mud_2))))
    (:`then_1`
      (`Timeline|TL_DelayBeforePause` :!via `PlayFromStart`
        (:`Finished`
          (`/Engine/EditorBlueprintResources/StandardMacros.IsValid` _vfx_mud
            (:`Is Valid`
              (`NiagaraComponent.SetPaused` _vfx_mud true))))))))

(event `self.ReceiveOnDespawnMole`
  (bind _vfx_mud (`self.VFX_Mud`))
  ;[1 0.4983 0.9027] On Destroy Mole
  (`|ExecutionSequence`
    (:`then_0`
      (`/Engine/EditorBlueprintResources/StandardMacros.IsValid` _vfx_mud
        (:`Is Valid`
          (`SceneComponent.SetVisibility` _vfx_mud false false))))))

(event `self.ReceiveOnMoleForcedDestroy`
  (bind _vfx_mud (`self.VFX_Mud`))
  ;[1 0.4983 0.9027] On Mole forced Destroy
  (`|ExecutionSequence`
    (:`then_0`
      (`/Engine/EditorBlueprintResources/StandardMacros.IsValid` _vfx_mud
        (:`Is Valid`
          (`SceneComponent.SetVisibility` _vfx_mud false false))))))

(fn `UserConstructionScript`)