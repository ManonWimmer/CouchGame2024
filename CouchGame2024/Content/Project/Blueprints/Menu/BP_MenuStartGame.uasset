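; BP_MenuStartGame is a menu trigger zone that starts the match when enough player balls roll into it.
; Sphere overlaps track unique BP_P_PlayerBall actors in an array and update a text actor's ready count, shown out of a hardcoded two.
; Once the required count is inside and at least four players are connected, a one-shot flag fires the WBP_MainMenu widget, a level sequence and a music fade-out.
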(event `self.Sphere.OnComponentBeginOverlap`
  (params (OverlappedComponent :type "PrimitiveComponent Object Reference") (OtherActor :type "Actor Object Reference") (OtherComp :type "PrimitiveComponent Object Reference") (OtherBodyIndex :type Integer) (bFromSweep :type Boolean) (SweepResult :type "HitResult Structure (by ref)"))
  (bind _returnvalue (subsystem `SoundSubsystem`))
  (bind _playersintrigger (`self.PlayersInTrigger`))
  (bind _returnvalue_2 (`KismetArrayLibrary.Array_Length` _playersintrigger))
  (bind _asbp_p_player_ball (cast `/Game/Project/Blueprints/Core/PlayerBall/BP_P_PlayerBall` OtherActor))
  (if (not (`KismetArrayLibrary.Array_Contains` _playersintrigger _asbp_p_player_ball))
    (`KismetArrayLibrary.Array_Add` _playersintrigger _asbp_p_player_ball)
    (`KismetSystemLibrary.PrintString` "Add player to trigger start game")
    (`TextRenderComponent.K2_SetText` (`TextRenderActor.TextRender` (`self.TextActor`)) (`KismetTextLibrary.Conv_StringToText` (`KismetStringLibrary.Concat_StrStr` "Players ready" (`KismetStringLibrary.Conv_IntToString` _returnvalue_2) "/2")))
    (if (and (and (>= _returnvalue_2 (`self.NumberOfPlayersNeededInTrigger`)) (>= (`LocalMultiplayerSubsystem.GetNumberOfPlayersConnected` (subsystem `LocalMultiplayerSubsystem`)) 4)) (not (`self.bHasStartedMatch`)))
      (set `self.bHasStartedMatch` true)
      (bind _returnvalue_3 (`|CreateWidget` "/Game/Project/UMG/WBP_MainMenu.WBP_MainMenu_C" (`GameplayStatics.GetPlayerController` 0)))
      (`UserWidget.AddToViewport` _returnvalue_3 0)
      (`MovieSceneSequencePlayer.Play` (`LevelSequenceActor.SequencePlayer` (`self.LevelSequenceActor`)))
      (`/Engine/EditorBlueprintResources/StandardMacros.IsValid` _returnvalue
        (:`Is Valid`
          (`SoundSubsystem.FadeOutMusic` _returnvalue))))))

(event `self.Sphere.OnComponentEndOverlap`
  (params (OverlappedComponent :type "PrimitiveComponent Object Reference") (OtherActor :type "Actor Object Reference") (OtherComp :type "PrimitiveComponent Object Reference") (OtherBodyIndex :type Integer))
  (bind _playersintrigger (`self.PlayersInTrigger`))
  (bind _asbp_p_player_ball (cast `/Game/Project/Blueprints/Core/PlayerBall/BP_P_PlayerBall` OtherActor))
  (if (`KismetArrayLibrary.Array_Contains` _playersintrigger _asbp_p_player_ball)
    (`KismetArrayLibrary.Array_RemoveItem` _playersintrigger _asbp_p_player_ball)
    (`KismetSystemLibrary.PrintString` "Remove  player from trigger start game")
    (`TextRenderComponent.K2_SetText` (`TextRenderActor.TextRender` (`self.TextActor`)) (`KismetTextLibrary.Conv_StringToText` (`KismetStringLibrary.Concat_StrStr` "Players ready" (`KismetStringLibrary.Conv_IntToString` (`KismetArrayLibrary.Array_Length` _playersintrigger)) "/2")))))

(fn `UserConstructionScript`)