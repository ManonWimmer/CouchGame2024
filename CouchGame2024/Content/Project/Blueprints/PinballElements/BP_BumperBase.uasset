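; Base pinball bumper Blueprint that supplies the visual and audio feedback for a bumper impact.
; BeginPlay caches the mesh's world X scale as the base scale.
; PlayBumperGamefeelEffectsBlueprint restarts a timeline that adds a uniform offset to that base scale when UseScaleEffect is enabled.
; The same event plays the impact sound through the sound subsystem if it is valid, independent of the scale toggle.
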(event `self.ReceiveBeginPlay`
  (bind _returnvalue_x (`KismetMathLibrary.BreakVector` (`SceneComponent.K2_GetComponentScale` (`self.StaticMesh`))))
  ;[0.4707 1 0.4036] Begin Play
  (set `self.BumperBaseScale` _returnvalue_x))

(event `self.PlayBumperGamefeelEffectsBlueprint`
  (bind _returnvalue (subsystem `SoundSubsystem`))
  ;[1 0.4697 0.8674] Bumper Gamefeel Effects
  (`|ExecutionSequence`
    (:`then_0`
      (if (`self.bUseScaleEffect`)
        (bind (_direction _scaleaddvalue) (`Timeline|TL_ScaleGamefeelEffect` :!via `PlayFromStart`)
          (:`Update`
            (bind _returnvalue_2 (+ _scaleaddvalue (`self.BumperBaseScale`)))
            (`SceneComponent.SetWorldScale3D` (`self.StaticMesh`) (`KismetMathLibrary.MakeVector` _returnvalue_2 _returnvalue_2 _returnvalue_2))))))
    (:`then_1`
      (`/Engine/EditorBlueprintResources/StandardMacros.IsValid` _returnvalue
        (:`Is Valid`
          (`SoundSubsystem.PlayBumperImpactSound` _returnvalue))))))

(fn `UserConstructionScript`)