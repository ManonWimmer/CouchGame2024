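; BP_BumperRond_Death is a round pinball bumper variant that animates its material's emissive glow when its element effects trigger.
; On BeginPlay it creates a dynamic instance of MAT_CircleBumper_Death on its static mesh.
; TriggerElementEffects extends the parent behavior by playing a timeline that drives the Emission Intensity parameter.
; A custom test event replays the same timeline.
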(event `self.ReceiveBeginPlay`
  ;[0.4707 1 0.4036] Begin Play
  (`parent.ReceiveBeginPlay`)
  (bind _returnvalue (`PrimitiveComponent.CreateDynamicMaterialInstance` (`self.StaticMesh`) 0 "/Game/Project/Assets/Art/03_Mat/Bumpers/MAT_CircleBumper_Death.MAT_CircleBumper_Death" "None"))
  (set `self.MaterialDynamic` _returnvalue))

(event `self.TriggerElementEffects`
  (bind _materialdynamic (`self.MaterialDynamic`))
  (`parent.TriggerElementEffects`)
  (bind (_direction _intensityvalue) (`Timeline|TL_IntensityEffect` :!via `PlayFromStart` :!label _label)
    (:`Update`
      _)
    (:`Finished`
      _))
  (`/Engine/EditorBlueprintResources/StandardMacros.IsValid` _materialdynamic
    (:`Is Valid`
      (`MaterialInstanceDynamic.SetScalarParameterValue` _materialdynamic "Emission Intensity" _intensityvalue))))

(event `CE_TestEffectIntesity`
  (goto _label :!via `PlayFromStart`))

(fn `UserConstructionScript`)