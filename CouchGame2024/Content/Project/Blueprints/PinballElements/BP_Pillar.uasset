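; Pinball pillar element that gives audio and visual feedback while grappling players gain points and when it is enabled, disabled or tricked.
; Gain point events fade a loop sound, show popcorn FX and tween the mesh scale, ending only when no player is still grappling.
; State events swap popcorn and empty meshes with a timed FX burst.
; Their SoundSubsystem cues are throttled by DoOnce and delay, with a Gate on disable.
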(event `self.ReceiveBeginPlay`
  ;[0.3742 1 0.4088] Begin Play
  (`|ExecutionSequence`
    (:`then_0`
      (`AudioComponent.Stop` (`self.SFX_GainPoint`)))))

(event `self.ReceiveOnStartGainPoint`
  (bind _asyncanim (`self.AsyncAnim`))
  (bind _sfx_gainpoint (`self.SFX_GainPoint`))
  (bind _fx_popcorn (`self.FX_Popcorn`))
  ;[1 0.3499 0.8853] Start / end Gain Point
  (`|ExecutionSequence`
    (:`then_0`
      (`/Engine/EditorBlueprintResources/StandardMacros.IsValid` _sfx_gainpoint
        (:`Is Valid`
          (`AudioComponent.Play` _sfx_gainpoint 0.0)
          (`AudioComponent.FadeIn` _sfx_gainpoint 0.5 1.0 0.0 "Linear")
          (`/Engine/EditorBlueprintResources/StandardMacros.IsValid` _fx_popcorn
            (:`Is Valid`
              (`SceneComponent.SetVisibility` _fx_popcorn true false))))))
    (:`then_1`
      (`/Engine/EditorBlueprintResources/StandardMacros.IsValid` _asyncanim
        (:`Is Valid`
          (`FCTweenBPAction.Stop` _asyncanim))
        (:`Is Not Valid`
          _))
      (bind (_asynctaskproxy _value) (`FCTweenBPActionVector.TweenVector` (`SceneComponent.RelativeScale3D` (`self.SM_Pillar`)) (4.3 4.3 4.3) 0.3 "OutQuad" 0.0 0.0 0.0 -1)
        (:`then`
          (set `self.AsyncAnim` _asynctaskproxy))
        (:`ApplyEasing`
          (`SceneComponent.SetRelativeScale3D` (`self.SM_Pillar`) _value))))))

(event `self.ReceiveOnEndGainPoint`
  (bind _fx_popcorn (`self.FX_Popcorn`))
  (bind _sfx_gainpoint (`self.SFX_GainPoint`))
  (bind _asyncanim (`self.AsyncAnim`))
  ;[1 0.3499 0.8853] Start / end Gain Point
  (if (<= (`self.GetNumberOfPlayersGrappling`) 0)
    (`|ExecutionSequence`
      (:`then_0`
        (`/Engine/EditorBlueprintResources/StandardMacros.IsValid` _sfx_gainpoint
          (:`Is Valid`
            (`AudioComponent.FadeOut` _sfx_gainpoint 0.5 0.0 "Linear")
            (`AudioComponent.StopDelayed` _sfx_gainpoint 0.5)
            (`/Engine/EditorBlueprintResources/StandardMacros.IsValid` _fx_popcorn
              (:`Is Valid`
                (`SceneComponent.SetVisibility` _fx_popcorn false false))))))
      (:`then_1`
        (`/Engine/EditorBlueprintResources/StandardMacros.IsValid` _asyncanim
          (:`Is Valid`
            (`FCTweenBPAction.Stop` _asyncanim)
            (`SceneComponent.SetRelativeScale3D` (`self.SM_Pillar`) (4.0 4.0 4.0))))))))

(event `self.ReceiveOnDisablePillar`
  (bind _returnvalue (subsystem `SoundSubsystem`))
  (bind _sm_pillar (`self.SM_Pillar`))
  (bind _meshpillarempty (`self.MeshPillarEmpty`))
  (bind _fx_popcorn (`self.FX_Popcorn`))
  ;[1 0.3499 0.8853] Enable / Disable Pillar
  (`|ExecutionSequence`
    (:`then_0`
      (`/Engine/EditorBlueprintResources/StandardMacros.Gate` true :!label _label
        (:`Exit`
          (`/Engine/EditorBlueprintResources/StandardMacros.DoOnce` false :!label _label_2
            (:`Completed`
              (`/Engine/EditorBlueprintResources/StandardMacros.IsValid` _returnvalue
                (:`Is Valid`
                  (`SoundSubsystem.PlayPillarOutSound` _returnvalue)
                  (`KismetSystemLibrary.Delay` 0.5)
                  (goto _label_2 :!via `Reset`))))))))
    (:`then_1`
      (goto _label :!via `Open`))
    (:`then_2`
      (`/Engine/EditorBlueprintResources/StandardMacros.IsValid` _fx_popcorn
        (:`Is Valid`
          (`SceneComponent.SetVisibility` _fx_popcorn true false)
          (`KismetSystemLibrary.Delay` (`self.PopcornTimeAnim`))
          (`SceneComponent.SetVisibility` _fx_popcorn false false))))
    (:`then_3`
      (`/Engine/EditorBlueprintResources/StandardMacros.IsValid` _sm_pillar
        (:`Is Valid`
          (`/Engine/EditorBlueprintResources/StandardMacros.IsValid` _meshpillarempty
            (:`Is Valid`
              (`StaticMeshComponent.SetStaticMesh` _sm_pillar _meshpillarempty))))))))

(event `self.ReceiveOnEnablePillar`
  (bind _returnvalue (subsystem `SoundSubsystem`))
  (bind _sm_pillar (`self.SM_Pillar`))
  (bind _meshpillarpopcorn (`self.MeshPillarPopcorn`))
  ;[1 0.3499 0.8853] Enable / Disable Pillar
  (`|ExecutionSequence`
    (:`then_0`
      (`/Engine/EditorBlueprintResources/StandardMacros.DoOnce` false :!label _label_3
        (:`Completed`
          (`/Engine/EditorBlueprintResources/StandardMacros.IsValid` _returnvalue
            (:`Is Valid`
              (`SoundSubsystem.PlayPillarInSound` _returnvalue)
              (`KismetSystemLibrary.Delay` 0.5)
              (goto _label_3 :!via `Reset`))))))
    (:`then_1`
      (`/Engine/EditorBlueprintResources/StandardMacros.IsValid` _sm_pillar
        (:`Is Valid`
          (`/Engine/EditorBlueprintResources/StandardMacros.IsValid` _meshpillarpopcorn
            (:`Is Valid`
              (if (== (`StaticMeshComponent.StaticMesh` _sm_pillar) (`self.MeshPillarEmpty`))
                (`SceneComponent.SetVisibility` (`self.FX_Popcorn`) true false)
                (`self.CE_DesacVFXPopcorn`))
              (`StaticMeshComponent.SetStaticMesh` _sm_pillar _meshpillarpopcorn))))))))

(event `CE_DesacVFXPopcorn`
  (`KismetSystemLibrary.Delay` (`self.PopcornTimeAnim`))
  (if (not (> (`self.GetNumberOfPlayersGrappling`) 0))
    (`SceneComponent.SetVisibility` (`self.FX_Popcorn`) false false)))

(event `self.ReceiveOnDisableTrickedZone`
  (bind _returnvalue (subsystem `SoundSubsystem`))
  (bind _sm_pillar (`self.SM_Pillar`))
  (bind _meshpillarempty (`self.MeshPillarEmpty`))
  (bind _fx_popcorn (`self.FX_Popcorn`))
  ;[1 0.3499 0.8853] Enable / Disable Pillar
  (`|ExecutionSequence`
    (:`then_0`
      (`/Engine/EditorBlueprintResources/StandardMacros.DoOnce` false :!label _label_4
        (:`Completed`
          (`/Engine/EditorBlueprintResources/StandardMacros.IsValid` _returnvalue
            (:`Is Valid`
              (`SoundSubsystem.PlayPillarBaitSound` _returnvalue)
              (`KismetSystemLibrary.Delay` 0.5)
              (goto _label_4 :!via `Reset`))))))
    (:`then_1`
      (`/Engine/EditorBlueprintResources/StandardMacros.IsValid` _fx_popcorn
        (:`Is Valid`
          (`SceneComponent.SetVisibility` _fx_popcorn true false)
          (`KismetSystemLibrary.Delay` (`self.PopcornTimeAnim`))
          (`SceneComponent.SetVisibility` _fx_popcorn false false))))
    (:`then_2`
      (`/Engine/EditorBlueprintResources/StandardMacros.IsValid` _sm_pillar
        (:`Is Valid`
          (`/Engine/EditorBlueprintResources/StandardMacros.IsValid` _meshpillarempty
            (:`Is Valid`
              (`StaticMeshComponent.SetStaticMesh` _sm_pillar _meshpillarempty))))))))

(fn `UserConstructionScript`)